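; Chance manager component for the card game that draws random cards and artifacts by gameplay tag, such as rarity.
; On BeginPlay it caches card and artifact pools from data tables.
; Draws filter and shuffle a pool, roll tags by cumulative weight, then take matches without repeats, excluding owned artifacts.
; Shortfalls are padded with duplicate picks or a ConsolationPrize row for cards, and a filler for artifacts.
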(event EventBeginPlay
  (CallFunction|GenerateAllCardsArray)
  (CallFunction|GenerateAllArifactsArray))

(fn GetRandomCardsbyDefaultTagWeights
  (params (Amount :type Integer))
  (bind _randomcards (CallFunction|GetRandomCardsbyTagWeights :TagWeights (Variables|Default|GetDefaultCardTagWeights) :Amount Amount))
  (return _randomcards))

(fn GetRandomCardsOfSpecificRarity
  (params (Rarity :type Gameplay%20Tag%20Structure) (Amount :type Integer))
  (bind _randomcards (CallFunction|GetRandomCardsbyTagWeights :TagWeights (Utilities|Map|MakeMap Rarity 1.0) :Amount Amount))
  (return _randomcards))

(fn GetTrueRandomCardsOfAnyRarity
  (params (Amount :type Integer))
  (bind _randomcards (CallFunction|GetRandomFilteredCards :Amount Amount :RequiredTags "(GameplayTags=((TagName=\"Rarity\")))"))
  (if (> Amount 1)
    (for _index (range 0 (- Amount 1))
      (Utilities|Array|Add (LocalVariables|GetLocalPickedCards) (Utilities|Array|Get(acopy) _randomcards _index)))
    (return (LocalVariables|GetLocalPickedCards))
    (else
      (return (Utilities|Array|MakeArray (Utilities|Array|Get(acopy) _randomcards))))))

(fn GetRandomArtifactsbyCustomTagWeights
  (params (TagWeights :type Map%20of%20Gameplay%20Tag%20Structures%20to%20Reals) (Amount :type Integer) (bExactMatch :type Boolean))
  (bind _remainingartifacts (CallFunction|GetRemainingArtifacts))
  (bind _output_get (LocalVariables|SetLocalArtifacts _remainingartifacts))
  (Utilities|Array|Shuffle _output_get)
  (bind _pickedtags (CallFunction|GetRandomTagsbyWeights TagWeights Amount))
  (for _array_element _pickedtags
    (bind (_bvalid _pickedartifact) (CallFunction|FindPickedTagAmongFilteredArtifacts _array_element (LocalVariables|GetLocalArtifacts) true))
    (if _bvalid
      (Utilities|Array|Add (LocalVariables|GetLocalPickedArtifacts) _pickedartifact)))
  (while (< (Utilities|Array|Length (LocalVariables|GetLocalPickedArtifacts)) Amount)
    (Utilities|Array|Add (LocalVariables|GetLocalPickedArtifacts) (LocalVariables|GetLocalFillerArtifact)))
  (return true (LocalVariables|GetLocalPickedArtifacts)))

(fn GetRandomArtifactsbyDefaultRarityWeights
  (params (Amount :type Integer))
  (bind (_bsuccess _pickedartifacts) (CallFunction|GetRandomArtifactsbyCustomTagWeights (Variables|Default|GetDefaultArtifactRarityWeights) Amount true))
  (return _bsuccess _pickedartifacts))

(fn GetFilteredCardswithAnyTag
  (params (Filter :type Gameplay%20Tag%20Container%20Structure) (Cards :type Array%20of%20F%20Card%20Structures) (bExactMatch :type Boolean))
  (for _array_element Cards
    (if (GameplayTags|HasAnyTags (Utilities|Struct|BreakFCard _array_element) Filter bExactMatch)
      (Utilities|Array|Add (LocalVariables|GetLocalFilteredCards) _array_element)))
  (return (LocalVariables|GetLocalFilteredCards)))

(fn GetRandomCardsbyTagWeights
  (params (TagWeights :type Map%20of%20Gameplay%20Tag%20Structures%20to%20Reals) (PossibleTags :type Gameplay%20Tag%20Container%20Structure) (RequiredTags :type Gameplay%20Tag%20Container%20Structure) (bExactMatch :type Boolean) (Amount :type Integer))
  (LocalVariables|SetLocalFilteredCards (Variables|Default|GetAllCards))
  (Utilities|FlowControl|Sequence
    (:then_0
      (if (> (Utilities|Array|Length (GameplayTags|BreakGameplayTagContainer RequiredTags)) 0)
        (bind _filteredcards (CallFunction|GetFilteredCardswithAllTags RequiredTags (LocalVariables|GetLocalFilteredCards) bExactMatch))
        (LocalVariables|SetLocalFilteredCards _filteredcards)))
    (:then_1
      (if (> (Utilities|Array|Length (GameplayTags|BreakGameplayTagContainer PossibleTags)) 0)
        (bind _filteredcards_2 (CallFunction|GetFilteredCardswithAnyTag PossibleTags (LocalVariables|GetLocalFilteredCards) bExactMatch))
        (LocalVariables|SetLocalFilteredCards _filteredcards_2)))
    (:then_2
      (if (> (Utilities|Array|Length (LocalVariables|GetLocalFilteredCards)) 0)
        (if (> (Utilities|Map|Length TagWeights) 0)
          (bind _keys (Utilities|Map|Keys TagWeights))
          (bind _filteredcards_3 (CallFunction|GetFilteredCardswithAnyTag (GameplayTags|MakeGameplayTagContainerfromArray _keys) (LocalVariables|GetLocalFilteredCards) bExactMatch))
          (bind _output_get (LocalVariables|SetLocalFilteredCards _filteredcards_3))
          (Utilities|Array|Shuffle _output_get)
          (bind _pickedtags (CallFunction|GetRandomTagsbyWeights TagWeights Amount))
          (for _array_element _pickedtags
            (bind (_bvalid _pickedcard) (CallFunction|FindPickedTagAmongFilteredCards _array_element (LocalVariables|GetLocalFilteredCards) true))
            (if _bvalid
              (Utilities|Array|Add (LocalVariables|GetLocalPickedCards) _pickedcard)))
          (if (> (Utilities|Array|Length (LocalVariables|GetLocalPickedCards)) 0)
            (LocalVariables|SetLocalPickedCardsWithDuplicates (LocalVariables|GetLocalPickedCards))
            (while (< (Utilities|Array|Length (LocalVariables|GetLocalPickedCardsWithDuplicates)) Amount)
              (Utilities|Array|Add (LocalVariables|GetLocalPickedCardsWithDuplicates) (.OutItem (Utilities|Array|Random (LocalVariables|GetLocalPickedCards)))))
            (return (LocalVariables|GetLocalPickedCardsWithDuplicates))
            (else
              _))
          (else
            (Utilities|Array|Shuffle (LocalVariables|GetLocalFilteredCards))
            (for _index (range 1 Amount)
              (Utilities|Array|Add (LocalVariables|GetLocalPickedCards) (Utilities|Array|Get(acopy) (LocalVariables|GetLocalFilteredCards) (Math|Integer|%(Integer) _index (Utilities|Array|Length (LocalVariables|GetLocalFilteredCards))))))
            (return (LocalVariables|GetLocalPickedCards)))))
      (bind _returnvalue (Utilities|GetDataTableRow "/Game/ShamanCardGame/Data/Cards/DT_Cards_Rewards.DT_Cards_Rewards" "ConsolationPrize")
        (:then
          (bind _structout (Utilities|Struct|SetmembersinFCard _returnvalue (Utilities|Struct|MakeDataTableRowHandle "/Game/ShamanCardGame/Data/Cards/DT_Cards_Rewards.DT_Cards_Rewards" "ConsolationPrize")))
          (while (< (Utilities|Array|Length (LocalVariables|GetLocalPickedCards)) Amount)
            (Utilities|Array|Add (LocalVariables|GetLocalPickedCards) _structout))
          (return (LocalVariables|GetLocalPickedCards)))
        (:RowNotFound
          (Development|PrintString "ERROR: Not enough valid card options, and no valid backup option" true true "(R=0.995000,G=0.000000,B=0.000000,A=1.000000)" 99.0)
          (return (LocalVariables|GetLocalPickedCards)))))))

(fn FindPickedTagAmongFilteredCards
  (params (PickedCardTag :type Gameplay%20Tag%20Structure) (FilteredCards :type Array%20of%20F%20Card%20Structures) (bPreventDuplicates :type Boolean))
  (bind (_arrayindex _arrayelement) (Utilities|Array|ReverseforEachLoop FilteredCards)
    (:LoopBody
      (if (GameplayTags|HasTag (Utilities|Struct|BreakFCard _arrayelement) PickedCardTag true)
        (LocalVariables|SetLocalPickedCard _arrayelement)
        (if bPreventDuplicates
          (Utilities|Array|RemoveIndex FilteredCards _arrayindex))
        (return true (LocalVariables|GetLocalPickedCard))))
    (:Completed
      (return false ""))))

(fn GetCardsbyDefaultRarityWeights
  (params (Amount :type Integer))
  (bind _randomcards (CallFunction|GetRandomCardsbyTagWeights :TagWeights (Variables|Default|GetDefaultCardTagWeights) :Amount Amount))
  (return _randomcards))

(fn GenerateAllCardsArray
  (Utilities|Array|Clear (Variables|Default|GetAllCards))
  (bind _rewardtables (Class|BPICardGameInstance|GetRewardTables(Message) (Game|GetGameInstance)))
  (for _array_element _rewardtables
    (bind _outrownames (DataTable|GetDataTableRowNames _array_element))
    (for _array_element_2 _outrownames
      (bind _returnvalue (Utilities|GetDataTableRow _array_element _array_element_2)
        (:then
          (bind _structout (Utilities|Struct|SetmembersinFCard _returnvalue (Utilities|Struct|MakeDataTableRowHandle _array_element _array_element_2)))
          (Utilities|Array|Add (Variables|Default|GetAllCards) _structout)))))
  (return (Variables|Default|GetAllCards)))

(fn GetRandomTagsbyWeights
  (params (WeightedTags :type Map%20of%20Gameplay%20Tag%20Structures%20to%20Reals) (Amount :type Integer))
  (bind _values (Utilities|Map|Values WeightedTags))
  (if (== (.MaxValue (Math|Float|MaxOfFloatArray _values)) (.MinValue (Math|Float|MinOfFloatArray _values))) ; If all weights are identical, simply pick random tags
    (while (< (Utilities|Array|Length (LocalVariables|GetLocalPickedTags)) Amount)
      (bind _keys (Utilities|Map|Keys WeightedTags))
      (Utilities|Array|Add (LocalVariables|GetLocalPickedTags) (.OutItem (Utilities|Array|Random _keys))))
    (return (LocalVariables|GetLocalPickedTags))
    (else
      (for _array_element _values
        (LocalVariables|SetLocalWeightSum (+ _array_element (LocalVariables|GetLocalWeightSum))))
      (while (< (Utilities|Array|Length (LocalVariables|GetLocalPickedTags)) Amount)
        (bind (_bsuccess _pickedtag) (CallFunction|PickTagfromWeightandWeightSum WeightedTags (LocalVariables|GetLocalWeightSum)))
        (if _bsuccess
          (Utilities|Array|Add (LocalVariables|GetLocalPickedTags) _pickedtag)))
      (return (LocalVariables|GetLocalPickedTags)))))

(fn PickTagfromWeightandWeightSum
  (params (WeightedTags :type Map%20of%20Gameplay%20Tag%20Structures%20to%20Reals) (WeightSum :type Float%20%28double-precision%29))
  (LocalVariables|SetLocalWeightSelection (Math|Random|RandomFloatinRange 0.0 WeightSum))
  (bind _keys (Utilities|Map|Keys WeightedTags))
  (for _array_element _keys
    (bind _output_get (LocalVariables|SetLocalWeightCount (+ (LocalVariables|GetLocalWeightCount) (.Value (Utilities|Map|Find WeightedTags _array_element)))))
    (if (>= _output_get (LocalVariables|GetLocalWeightSelection))
      (return true _array_element)))
  (return false ""))

(fn GenerateAllArifactsArray
  (for _array_element (Variables|Default|GetArtifactTables)
    (bind _outrownames (DataTable|GetDataTableRowNames _array_element))
    (for _array_element_2 _outrownames
      (bind _returnvalue (Utilities|GetDataTableRow _array_element _array_element_2)
        (:then
          (Utilities|Array|Add (Variables|Default|GetAllArtifacts) _returnvalue))))
    (return (Variables|Default|GetAllArtifacts))))

(fn FindPickedTagAmongFilteredArtifacts
  (params (PickedTag :type Gameplay%20Tag%20Structure) (FilteredArtifacts :type Array%20of%20F%20Status%20Structures) (bPreventDuplicates :type Boolean))
  (for (_array_element _array_index) FilteredArtifacts
    (if (GameplayTags|HasTag (Utilities|Struct|BreakFStatus _array_element) PickedTag true)
      (LocalVariables|SetLocalPickedArtifact _array_element)
      (if bPreventDuplicates
        (Utilities|Array|RemoveIndex FilteredArtifacts _array_index))
      (return true (LocalVariables|GetLocalPickedArtifact))))
  (return false ""))

(fn GetFilteredCardswithAllTags
  (params (Filter :type Gameplay%20Tag%20Container%20Structure) (Cards :type Array%20of%20F%20Card%20Structures) (bExactMatch :type Boolean))
  (for _array_element Cards
    (if (GameplayTags|HasAllTags (Utilities|Struct|BreakFCard _array_element) Filter bExactMatch)
      (Utilities|Array|Add (LocalVariables|GetLocalFilteredCards) _array_element)))
  (return (LocalVariables|GetLocalFilteredCards)))

(fn GetRemainingArtifacts
  (LocalVariables|SetLocalRemainingArtifacts (Variables|Default|GetAllArtifacts))
  (bind _artifacts (Class|BPICardGameInstance|GetArtifactsfromInstance(Message) (Game|GetGameInstance)))
  (for _array_element _artifacts
    (for _array_element_2 (Variables|Default|GetAllArtifacts)
      (if (== (.StatusClass (Utilities|Struct|BreakFStatus _array_element_2)) (.StatusClass (Utilities|Struct|BreakFStatus _array_element)))
        (Utilities|Array|RemoveItem (LocalVariables|GetLocalRemainingArtifacts) _array_element_2))))
  (return (LocalVariables|GetLocalRemainingArtifacts)))

(fn GetRandomFilteredCards
  (params (Amount :type Integer) (PossibleTags :type Gameplay%20Tag%20Container%20Structure) (RequiredTags :type Gameplay%20Tag%20Container%20Structure) (bExactMatch :type Boolean))
  (bind _randomcards (CallFunction|GetRandomCardsbyTagWeights (LocalVariables|GetLocalEmptyWeights) PossibleTags RequiredTags bExactMatch Amount))
  (return _randomcards))