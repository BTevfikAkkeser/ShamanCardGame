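; Attack pattern component for the Spider Queen enemy in the card game, overriding how the next card is chosen.
; When the owning minion is alone on its minion track and the pattern is past its second step, it resets the pattern index so the sequence restarts.
; It then defers to the parent selection, bringing back the early summoning ability the pattern is assumed to contain.
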(fn GetNextCard
  ;[0 0 0] If the Spider Queen is the only remaining enemy it will restart its attack pattern (which is assumed to have a summoning ability set early on)
  (bind _asbp_minion (Utilities|Casting|CastToBP_Minion (Components|GetOwner)))
  (if (and (== (Utilities|Array|Length (Variables|/Game/ShamanCardGame/Blueprints/Core/BP_MinionTrack.BP_MinionTrack_C|GetMinions (Variables|/Game/ShamanCardGame/Blueprints/Core/BP_Minion.BP_Minion_C|GetMinionTrack _asbp_minion))) 1) (> (Variables|Default|GetPatternIndex) 1))
    (Variables|Default|SetPatternIndex -1))
  (bind _card (|CallParentFunction))
  (return _card))