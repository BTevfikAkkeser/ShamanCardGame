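; BP_RewardHolder is an actor that holds BP_Status components as rewards for the card game's reward screen.
; AddToStatus increases an existing status or adds a new component of that class, with the player's WBPRewardScreen as its UI owner.
; It listens on the global dispatcher hub for Event.CloseRewardScreen and destroys its status components in response.
; The remaining targeting, identity and status functions are stubs returning empty or failure values.
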(event EventBeginPlay
  (CallFunction|BindEventtoGlobalDispatcherHub self "(TagName=\"Event.CloseRewardScreen\")"))

(event EventRunEvent
  (params (EventTag :type Gameplay%20Tag%20Structure) (CallingObject :type Object%20Object%20Reference%20%28by%20ref%29) (bGlobal :type Boolean) (Payload :type Object%20Object%20Reference%20%28by%20ref%29) (CallTags :type Gameplay%20Tag%20Container%20Structure%20%28by%20ref%29))
  (|SwitchGameplayTag EventTag
    (:Event.CloseRewardScreen
      (for _array_element (Actor|GetComponentsByClass "/Game/ShamanCardGame/Blueprints/Statuses/BP_Status.BP_Status_C")
        (Components|DestroyComponent _array_element)))))

(fn ConstructionScript)

(fn AddtoStatus
  (params (StatusClass :type BP%20Status%20Class%20Reference) (Amount :type Integer) (bShowSplash :type Boolean) (Payload :type Object%20Object%20Reference))
  (bind _returnvalue (Actor|GetComponentbyClass StatusClass))
  (Utilities|IsValid _returnvalue
    (:Is%20Valid
      (bind _newvalue (Default|AddStatusValue _returnvalue Amount false false false Payload))
      (return _newvalue))
    (:Is%20Not%20Valid
      (if (or (> Amount 0) (Utilities|GetClassDefaults StatusClass))
        (bind _cardplayer (CallFunction|GetCardPlayer))
        (bind _returnvalue_2 (Game|AddComponentbyClass StatusClass 0 (Variables|/Game/ShamanCardGame/Widgets/WBP_Layout_RLDB.WBP_Layout_RLDB_C|GetWBP_RewardScreen (Variables|/Game/ShamanCardGame/Blueprints/Core/BP_CardPlayer.BP_CardPlayer_C|GetPlayerUI _cardplayer))))
        (Default|AddStatusValue _returnvalue_2 Amount false false true Payload)
        (return Amount)
        (else
          (return 0))))))

(fn AttemptMarkTarget
  (params (ValidTargets :type Gameplay%20Tag%20Container%20Structure))
  (return false))

(fn CheckifValidTarget
  (params (ValidTargets :type Gameplay%20Tag%20Container%20Structure))
  (return false))

(fn GetFriendlyName
  (return ""))

(fn GetMinionUniqueId
  (return ""))

(fn GetPriority
  (return 0.0))

(fn GetPuppet
  (return 0))

(fn GetStatusMax
  (params (Status :type BP%20Status%20Class%20Reference))
  (return false 0))

(fn GetStatusValue
  (params (Status :type BP%20Status%20Class%20Reference))
  (return false 0))

(fn MarkTarget
  (return false))

(fn SetStatusMax
  (params (Status :type BP%20Status%20Class%20Reference) (NewMax :type Integer))
  (return false))

(fn SubtractfromStatus
  (params (StatusClass :type BP%20Status%20Class%20Reference) (Amount :type Integer) (bShowSplash :type Boolean) (Payload :type Object%20Object%20Reference))
  (return 0))