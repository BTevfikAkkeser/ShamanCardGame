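; Component that moves cards between a card player's piles in response to gameplay-tagged card events such as discard, draw, exhaust, generate and reshuffle.
; RunCardTransferEvent switches on the event tag, picks a target pile, then ResolveTransfer updates both piles and spawns a BP_Action_CardTransfer actor.
; Generate, return-to-hand, reshuffle and active discards also queue action events in the global dispatcher hub.
; An Interrupt flag makes it skip the next event.
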(event EventBeginPlay
  (CallFunction|BindMultipleEventstoGlobalDispatcherHub self "(GameplayTags=((TagName=\"Event.Card.Discard\"),(TagName=\"Event.Card.Exhaust\"),(TagName=\"Event.Card.Void\"),(TagName=\"Event.Card.Destroy\"),(TagName=\"Event.Card.Draw\"),(TagName=\"Event.Card.PrePlay\"),(TagName=\"Event.Card.Generate\"),(TagName=\"Event.Card.ReturnToHand\"),(TagName=\"Event.Reshuffle\")))"))

(event EventRunEvent
  (params (EventTag :type Gameplay%20Tag%20Structure) (CallingObject :type Object%20Object%20Reference%20%28by%20ref%29) (bGlobal :type Boolean) (Payload :type Object%20Object%20Reference%20%28by%20ref%29) (CallTags :type Gameplay%20Tag%20Container%20Structure%20%28by%20ref%29))
  (bind _asbp_card (Utilities|Casting|CastToBP_Card CallingObject)
    (:then
      _)
    (:CastFailed
      _))
  (CallFunction|RunCardTransferEvent EventTag _asbp_card CallTags))

(event EventInterrupt
  (Variables|Default|SetbInterrupt true))

(event EventCancelInterruption
  (Variables|Default|SetbInterrupt false))

(fn ResolveTransfer
  (params (Card :type BP%20Card%20Object%20Reference) (SourcePileTag :type Gameplay%20Tag%20Structure) (TargetPileTag :type Gameplay%20Tag%20Structure))
  (bind _cardplayer (CallFunction|GetCardPlayerPure))
  (bind (_bsuccess _pile) (Default|GetPilewithPileTag _cardplayer SourcePileTag))
  (if _bsuccess
    (Default|RequestRemoveCardfromPile _pile Card))
  (Default|AttemptAddExistingCard (.Pile (Default|GetPilewithPileTag (CallFunction|GetCardPlayerPure) TargetPileTag)) Card)
  (Game|SpawnActorfromClass "/Game/ShamanCardGame/Blueprints/CardActions/BP_Action_CardTransfer.BP_Action_CardTransfer_C" (Math|Transform|MakeTransform "0, 0, 0" "0, 0, 0" "1.000000,1.000000,1.000000") "AlwaysSpawn" "OverrideRootScale" 0 Card SourcePileTag TargetPileTag 0.1 0)
  (return true))

(fn ReturnCardtoHand
  (params (Card :type BP%20Card%20Object%20Reference%20%28by%20ref%29) (CallingObject :type Object%20Object%20Reference%20%28by%20ref%29))
  (Default|AttemptAddExistingCard (Variables|/Game/ShamanCardGame/Blueprints/Core/BP_CardPlayer.BP_CardPlayer_C|GetBP_PileComponent_Hand (CallFunction|GetCardPlayerPure)) Card)
  (CallFunction|QueueEventinGlobalDispatcherHub "(TagName=\"Event.Action.ReturnCardToHand\")" Card 0 0.1)
  (return))

(fn GenerateCard
  (params (Card :type BP%20Card%20Object%20Reference) (DisplayTime :type Float%20%28double-precision%29))
  (if (GameplayTags|MatchesAnyTags (Variables|/Game/ShamanCardGame/Blueprints/Core/BP_Card.BP_Card_C|GetCurrentPile Card) (LocalVariables|GetLocalPileTagsToAnimate) true)
    (CallFunction|QueueEventinGlobalDispatcherHub "(TagName=\"Event.Action.GenerateCard\")" Card 0 DisplayTime)
    (Game|SpawnActorfromClass :Class "/Game/ShamanCardGame/Blueprints/CardActions/BP_Action_CardTransfer.BP_Action_CardTransfer_C" :CollisionHandlingOverride "AlwaysSpawn" :TransformScaleMethod "OverrideRootScale" :Card Card :TargetPile (Variables|/Game/ShamanCardGame/Blueprints/Core/BP_Card.BP_Card_C|GetCurrentPile Card) :EndDelay (Variables|Default|GetCardTransferFrequency) :Instigator 0)
    (return)
    (else
      (return))))

(fn Reshuffle
  (CallFunction|QueueEventinGlobalDispatcherHub "(TagName=\"Event.Action.Reshuffle\")" self 0 -1.0)
  (Game|SpawnActorfromClass "/Game/ShamanCardGame/Blueprints/CardActions/BP_Action_Reshuffle.BP_Action_Reshuffle_C" (Math|Transform|MakeTransform "0, 0, 0" "0, 0, 0" "1.000000,1.000000,1.000000") "AlwaysSpawn" "OverrideRootScale" 0 (Variables|/Game/ShamanCardGame/Blueprints/Piles/BP_PileComponent.BP_PileComponent_C|GetCards (Variables|/Game/ShamanCardGame/Blueprints/Core/BP_CardPlayer.BP_CardPlayer_C|GetBP_PileComponent_Discard (CallFunction|GetCardPlayerPure))) 0.2 0)
  (return))

(fn RunCardTransferEvent
  (params (EventTag :type Gameplay%20Tag%20Structure) (Card :type BP%20Card%20Object%20Reference%20%28by%20ref%29) (CallTags :type Gameplay%20Tag%20Container%20Structure))
  (if (Variables|Default|GetbInterrupt)
    (Variables|Default|SetbInterrupt false)
    (return)
    (else
      (|SwitchGameplayTag EventTag
        (:Event.Card.Discard
          (Variables|Default|SetCurrentTargetPile "(TagName=\"Pile.Discard\")")
          (|SwitchGameplayTagContainer CallTags
            (:Default
              _)
            (:%28GameplayTags=%28%28TagName="Flag.Active"%29%29%29
              (CallFunction|QueueEventinGlobalDispatcherHub "(TagName=\"Event.Action.FlickCard\")" Card 0 0.2))
            (:%28GameplayTags=%28%28TagName="Flag.Passive"%29%29%29
              _))
          (CallFunction|ResolveTransfer Card (Variables|/Game/ShamanCardGame/Blueprints/Core/BP_Card.BP_Card_C|GetCurrentPile Card) (Variables|Default|GetCurrentTargetPile))
          (return))
        (:Event.Card.Draw
          (Variables|Default|SetCurrentTargetPile "(TagName=\"Pile.Hand\")"))
        (:Event.Card.Exhaust
          (Variables|Default|SetCurrentTargetPile "(TagName=\"Pile.Exhaust\")"))
        (:Event.Card.Void
          (Variables|Default|SetCurrentTargetPile "(TagName=\"Pile.Void\")"))
        (:Event.Card.Destroy
          (Variables|Default|SetCurrentTargetPile "(TagName=\"Pile.Destroy\")"))
        (:Event.Card.PrePlay
          (Utilities|Array|RemoveItem (Variables|/Game/ShamanCardGame/Blueprints/Piles/BP_PileComponent.BP_PileComponent_C|GetCards (Actor|GetComponentbyClass (Components|GetOwner) "/Game/ShamanCardGame/Blueprints/Piles/BP_PileComponent_Hand.BP_PileComponent_Hand_C")) Card)
          (return))
        (:Event.Card.Generate
          (CallFunction|GenerateCard Card (Math|Float|SelectFloat 1.5 0.4 (GameplayTags|HasTag CallTags "(TagName=\"Flag.Slow\")")))
          (return))
        (:Event.Card.ReturnToHand
          (CallFunction|ReturnCardtoHand Card Card)
          (return))
        (:Event.Reshuffle
          (CallFunction|Reshuffle)
          (return)))
      (CallFunction|ResolveTransfer Card (Variables|/Game/ShamanCardGame/Blueprints/Core/BP_Card.BP_Card_C|GetCurrentPile Card) (Variables|Default|GetCurrentTargetPile))
      (return))))

(fn GetFriendlyName
  (return ""))

(fn GetPriority
  (return (Variables|Default|GetPriority)))