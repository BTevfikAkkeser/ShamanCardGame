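; Local event dispatcher component for the card game that extends a parent dispatcher hub and can relay tag-based events to the global hub.
; On BeginPlay it caches the hub component from BP_GlobalDispatcherHub.
; All CallEvent variants, with optional payload and call tags, funnel into ResolveCallEvent, which fires locally only, or also globally before or after.
; Bind and unbind maintain an Empty flag so local dispatch is skipped without listeners.
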(event EventBeginPlay
  (bind _returnvalue (Actor|GetActorOfClass "/Game/ShamanCardGame/Blueprints/Core/BP_GlobalDispatcherHub.BP_GlobalDispatcherHub_C"))
  (Variables|Default|SetGlobalDispatcherHubRef (Variables|/Game/ShamanCardGame/Blueprints/Core/BP_GlobalDispatcherHub.BP_GlobalDispatcherHub_C|GetBP_DispatcherHubComponent _returnvalue)))

(fn CallEvent
  (params (EventTag :type Gameplay%20Tag%20Structure) (CallingObject :type Object%20Object%20Reference%20%28by%20ref%29) (CallSpecificObject :type Object%20Object%20Reference) (AlsoCallGlobal :type ECallGlobal%20Enum :default "NewEnumerator0"))
  (bind _bsuccess (CallFunction|ResolveCallEvent EventTag CallingObject CallSpecificObject AlsoCallGlobal (Game|GetGameInstance) (Variables|Default|GetBlankContainer)))
  (return _bsuccess))

(fn CallEventwithCallTags
  (params (EventTag :type Gameplay%20Tag%20Structure) (CallingObject :type Object%20Object%20Reference%20%28by%20ref%29) (CallSpecificObject :type Object%20Object%20Reference) (AlsoCallGlobal :type ECallGlobal%20Enum :default "NewEnumerator0") (CallTags :type Gameplay%20Tag%20Container%20Structure))
  (bind _bsuccess (CallFunction|ResolveCallEvent EventTag CallingObject CallSpecificObject AlsoCallGlobal (Game|GetGameInstance) CallTags))
  (return _bsuccess))

(fn ResolveCallEvent
  (params (EventTag :type Gameplay%20Tag%20Structure) (CallingObject :type Object%20Object%20Reference%20%28by%20ref%29) (CallSpecificObject :type Object%20Object%20Reference) (AlsoCallGlobal :type ECallGlobal%20Enum :default "NewEnumerator0") (Payload :type Object%20Object%20Reference%20%28by%20ref%29) (CallTags :type Gameplay%20Tag%20Container%20Structure%20%28by%20ref%29))
  (switch Utilities|FlowControl|Switch|SwitchonECallGlobal AlsoCallGlobal
    (:NewEnumerator0
      _)
    (:NewEnumerator1
      (CallFunction|ResolveCallEvent (Variables|Default|GetGlobalDispatcherHubRef) EventTag CallingObject CallSpecificObject AlsoCallGlobal Payload CallTags))
    (:NewEnumerator2
      (if (Variables|Default|GetbEmpty)
        _
        (else
          (|CallParentFunction EventTag CallingObject CallSpecificObject AlsoCallGlobal Payload CallTags)))
      (bind _bsuccess (CallFunction|ResolveCallEvent (Variables|Default|GetGlobalDispatcherHubRef) EventTag CallingObject CallSpecificObject AlsoCallGlobal Payload CallTags))
      (return _bsuccess)))
  (if (Variables|Default|GetbEmpty)
    (return true)
    (else
      (bind _bsuccess_2 (|CallParentFunction EventTag CallingObject CallSpecificObject AlsoCallGlobal Payload CallTags))
      (return _bsuccess_2))))

(fn CallEventwithPayload
  (params (EventTag :type Gameplay%20Tag%20Structure) (CallingObject :type Object%20Object%20Reference%20%28by%20ref%29) (CallSpecificObject :type Object%20Object%20Reference) (AlsoCallGlobal :type ECallGlobal%20Enum :default "NewEnumerator0") (Payload :type Object%20Object%20Reference%20%28by%20ref%29))
  (bind _bsuccess (CallFunction|ResolveCallEvent EventTag CallingObject CallSpecificObject AlsoCallGlobal Payload (Variables|Default|GetBlankContainer)))
  (return _bsuccess))

(fn CallEventwithPayloadandCallTags
  (params (EventTag :type Gameplay%20Tag%20Structure) (CallingObject :type Object%20Object%20Reference%20%28by%20ref%29) (CallSpecificObject :type Object%20Object%20Reference) (AlsoCallGlobal :type ECallGlobal%20Enum :default "NewEnumerator0") (Payload :type Object%20Object%20Reference%20%28by%20ref%29) (CallTags :type Gameplay%20Tag%20Container%20Structure))
  (bind _bsuccess (CallFunction|ResolveCallEvent EventTag CallingObject CallSpecificObject AlsoCallGlobal Payload CallTags))
  (return _bsuccess))

(fn BindEventtoHub
  (params (EventHolder :type Object%20Object%20Reference) (EventTag :type Gameplay%20Tag%20Structure))
  (|CallParentFunction EventHolder EventTag)
  (Variables|Default|SetbEmpty false)
  (return))

(fn UnbindEventfromHub
  (params (EventHolder :type Object%20Object%20Reference) (EventTag :type Gameplay%20Tag%20Structure))
  (|CallParentFunction EventHolder EventTag)
  (Variables|Default|SetbEmpty (Utilities|Map|IsEmpty (Variables|Default|GetEventLists)))
  (return))