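; Component for the Shaman card game that stores payloads in a map keyed by identifier, so they can be retrieved later.
; AddPayload registers a payload, printing a yellow warning and overriding the existing entry when the identifier is already taken.
; AccessPayload returns a success flag with the value, optionally removing the entry on access for one-time consumption.
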(fn AddPayload
  (params (Identifier :type String) (Payload :type Object%20Object%20Reference%20%28by%20ref%29))
  (if (Utilities|Map|Contains (Variables|Default|GetPayloads) Identifier)
    (Development|PrintString (Utilities|String|Append "WARNING: Adding Payload " (Utilities|GetDisplayName Payload) " with Identifier " Identifier " to Payload Holder Component " (Utilities|GetDisplayName self) ", which already exists. Overriding existing payload.") true true "(R=1.000000,G=1.000000,B=0.000000,A=1.000000)"))
  (Utilities|Map|Add (Variables|Default|GetPayloads) Identifier Payload)
  (return))

(fn AccessPayload
  (params (Identifier :type String) (bDestroyAfterAccess :type Boolean))
  (bind _payloads (Variables|Default|GetPayloads))
  (bind (_value _returnvalue) (Utilities|Map|Find _payloads Identifier))
  (if _returnvalue
    (if bDestroyAfterAccess
      (LocalVariables|SetLocalPayload _value)
      (Utilities|Map|Remove (Variables|Default|GetPayloads) Identifier)
      (return true (LocalVariables|GetLocalPayload))
      (else
        (return true _value)))
    (else
      (return false 0))))