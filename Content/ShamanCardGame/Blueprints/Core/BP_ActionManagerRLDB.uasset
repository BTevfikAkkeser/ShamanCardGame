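; Action manager for the card game that plays queued actions one after another, telling each to animate.
; Actions sit in a fixed-size ring buffer with separate fill and play counters, printing an error on overflow.
; Playback waits for a valid next action and caps starts per tick; finished actions are asked to destroy themselves before the next plays.
; QueueDelay spawns a BP_ActionRLDB with an end delay.
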(event Custom|AttemptToPlayNextAction
  (Utilities|DelayWhile (or (not (Utilities|IsValid (Utilities|Array|Get(acopy) (Variables|Default|GetActionQueue) (CallFunction|GetNextQueueIndex (Variables|Default|GetQueueCounter))))) (>= (Variables|Default|GetActionsThisTick) (Variables|Default|GetMaxActionsPerTick)))
    (:Continue
      (Variables|Default|SetActionsThisTick (+ (Variables|Default|GetActionsThisTick) 1))
      (bind _output_get (Variables|Default|SetQueueCounter (CallFunction|GetNextQueueIndex (Variables|Default|GetQueueCounter))))
      (Class|BPICardAction|AnimateAction(Message) (Utilities|Array|Get(acopy) (Variables|Default|GetActionQueue) _output_get) self))))

(event Custom|QueueAction
  (params (Action :type Object%20Object%20Reference))
  (bind _output_get (Variables|Default|SetFillCounter (CallFunction|GetNextQueueIndex (Variables|Default|GetFillCounter))))
  (if (not (Utilities|IsValid (Utilities|Array|Get(acopy) (Variables|Default|GetActionQueue) _output_get)))
    (Utilities|Array|SetArrayElem (Variables|Default|GetActionQueue) _output_get Action)
    (else
      (Development|PrintString "ERROR: Action Overflow" true true "(R=1.000000,G=0.000000,B=0.000000,A=1.000000)" 999.0))))

(event EventTick
  (params (DeltaSeconds :type Float%20%28single-precision%29))
  (Variables|Default|SetActionsThisTick 0))

(event EventBeginPlay
  (Utilities|Array|Resize (Variables|Default|GetActionQueue) (Variables|Default|GetQueueSize))
  (CallFunction|AttempttoPlayNextAction))

(event EventProceedfromOngoingAction
  (params (OngoingAction :type Object%20Object%20Reference))
  (Class|BPICardAction|AttemptDestroyAction(Message) OngoingAction)
  (CallFunction|AttempttoPlayNextAction))

(fn ConstructionScript)

(fn GetNextQueueIndex
  (params (CurrentIndex :type Integer))
  (return (Math|Integer|%(Integer) (+ CurrentIndex 1) (Utilities|Array|Length (Variables|Default|GetActionQueue)))))

(fn QueueDelay
  (params (Delay :type Float%20%28double-precision%29))
  (Game|SpawnActorfromClass "/Game/ShamanCardGame/Blueprints/CardActions/BP_ActionRLDB.BP_ActionRLDB_C" (Math|Transform|MakeTransform "0, 0, 0" "0, 0, 0" "1.000000,1.000000,1.000000") "AlwaysSpawn" "OverrideRootScale" 0 Delay 0)
  (return))