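; Card targeting mode that lets the player hand-pick one card from the pile component specified by the card effect.
; FindValidTargets finds no targets for previews or empty piles; otherwise it puts the hand in selection mode and fills the card selector list.
; It reports success immediately, then the list's confirm callback unbinds itself, clears selection mode and broadcasts the chosen card as the input target.
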(event Custom|ValidateAndTransferSelectedCard
  (params (Card :type BP%20Card%20Object%20Reference))
  (EventDispatchers|UnbindEventfromOnReturnSelectedCard (stale Custom|BindToCardConfirm CardList) (delegate Custom|ValidateAndTransferSelectedCard))
  (bind _returnvalue (Actor|GetActorOfClass "/Game/ShamanCardGame/Blueprints/Core/BP_CardPlayer.BP_CardPlayer_C"))
  (Variables|/Game/ShamanCardGame/Widgets/WBP_CardHand.WBP_CardHand_C|SetbSelectionMode (Variables|/Game/ShamanCardGame/Widgets/WBP_Layout_RLDB.WBP_Layout_RLDB_C|GetWBP_Hand (Variables|/Game/ShamanCardGame/Blueprints/Core/BP_CardPlayer.BP_CardPlayer_C|GetPlayerUI _returnvalue)) false)
  (Default|CallOnInputTargetsReceived (Utilities|Array|MakeArray Card)))

(event Custom|BindToCardConfirm
  (params (CardList :type WBP%20Card%20Selector%20List%20Object%20Reference))
  (EventDispatchers|BindEventtoOnReturnSelectedCard CardList (delegate Custom|ValidateAndTransferSelectedCard)))

(fn FindValidTargets
  (params (SpecifiedTargets :type Array%20of%20Actor%20Object%20References) (CardEffect :type F%20Card%20Effect%20Structure) (Card :type BP%20Card%20Object%20Reference) (bPreview :type Boolean))
  (if bPreview
    (return false 0)
    (else
      (bind _asbp_pile_component (Utilities|Casting|CastToBP_PileComponentClass (CallFunction|GetEffectTargetComponent CardEffect))
        (:then
          (bind _returnvalue (Actor|GetActorOfClass "/Game/ShamanCardGame/Blueprints/Core/BP_CardPlayer.BP_CardPlayer_C"))
          (if (> (Utilities|Array|Length (Variables|/Game/ShamanCardGame/Blueprints/Piles/BP_PileComponent.BP_PileComponent_C|GetCards (Actor|GetComponentbyClass _returnvalue _asbp_pile_component))) 0)
            (Variables|/Game/ShamanCardGame/Widgets/WBP_CardHand.WBP_CardHand_C|SetbSelectionMode (Variables|/Game/ShamanCardGame/Widgets/WBP_Layout_RLDB.WBP_Layout_RLDB_C|GetWBP_Hand (Variables|/Game/ShamanCardGame/Blueprints/Core/BP_CardPlayer.BP_CardPlayer_C|GetPlayerUI _returnvalue)) true)
            (CallFunction|BindtoCardConfirm (Variables|/Game/ShamanCardGame/Widgets/WBP_Layout_RLDB.WBP_Layout_RLDB_C|GetWBP_CardSelectorList (Variables|/Game/ShamanCardGame/Blueprints/Core/BP_CardPlayer.BP_CardPlayer_C|GetPlayerUI _returnvalue)))
            (Default|UpdateCardList (Variables|/Game/ShamanCardGame/Widgets/WBP_Layout_RLDB.WBP_Layout_RLDB_C|GetWBP_CardSelectorList (Variables|/Game/ShamanCardGame/Blueprints/Core/BP_CardPlayer.BP_CardPlayer_C|GetPlayerUI _returnvalue)) (Variables|/Game/ShamanCardGame/Blueprints/Piles/BP_PileComponent.BP_PileComponent_C|GetCards (Actor|GetComponentbyClass _returnvalue _asbp_pile_component)) "Choose a Card")
            (return true 0)
            (else
              (return false 0))))
        (:CastFailed
          (return false 0))))))