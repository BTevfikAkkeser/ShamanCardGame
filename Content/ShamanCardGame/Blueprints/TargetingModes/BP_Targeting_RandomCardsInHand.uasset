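; A card targeting mode that picks random cards from the hand of the card player returned by GetCardPlayer.
; FindValidTargets gathers hand cards matching any of the effect's gameplay tags, or every card when the effect has none.
; It then draws random picks without repeats until it reaches the effect's EffectValue or runs out, and reports whether any target was found.
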(fn FindValidTargets
  (params (SpecifiedTargets :type Array%20of%20Actor%20Object%20References) (CardEffect :type F%20Card%20Effect%20Structure) (Card :type BP%20Card%20Object%20Reference) (bPreview :type Boolean))
  (bind _cardplayer (CallFunction|GetCardPlayer))
  (for _array_element (Variables|/Game/ShamanCardGame/Blueprints/Piles/BP_PileComponent.BP_PileComponent_C|GetCards (Actor|GetComponentbyClass _cardplayer "/Game/ShamanCardGame/Blueprints/Piles/BP_PileComponent_Hand.BP_PileComponent_Hand_C"))
    (if (or (== (Utilities|Array|Length (.gameplaytags (CallFunction|GetEffectGameplayTags CardEffect))) 0) (GameplayTags|HasAnyTags (CallFunction|GetEffectGameplayTags CardEffect) (Variables|/Game/ShamanCardGame/Blueprints/Core/BP_GameplayTagComponent.BP_GameplayTagComponent_C|GetGameplayTags (Actor|GetComponentbyClass _array_element "/Game/ShamanCardGame/Blueprints/Core/BP_GameplayTagComponent.BP_GameplayTagComponent_C"))))
      (Utilities|Array|Add (LocalVariables|GetLocalValidTargets) _array_element)))
  (while (and (> (Utilities|Array|Length (LocalVariables|GetLocalValidTargets)) 0) (< (Utilities|Array|Length (LocalVariables|GetLocalSelectedTargets)) (.EffectValue (Utilities|Struct|BreakFCardEffect CardEffect))))
    (bind _output_get (LocalVariables|SetLocalTarget (.OutItem (Utilities|Array|Random (LocalVariables|GetLocalValidTargets)))))
    (Utilities|Array|Add (LocalVariables|GetLocalSelectedTargets) _output_get)
    (Utilities|Array|RemoveItem (LocalVariables|GetLocalValidTargets) (LocalVariables|GetLocalTarget)))
  (return (> (Utilities|Array|Length (LocalVariables|GetLocalSelectedTargets)) 0) (LocalVariables|GetLocalSelectedTargets)))