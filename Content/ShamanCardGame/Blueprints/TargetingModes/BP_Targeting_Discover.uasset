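; Discover targeting mode for card effects that offers generated cards on a reward screen and returns the pick as the effect's target.
; For pile effects outside preview, it takes one specified data-table card or rolls three through the chance manager, optionally rarity-weighted or filtered to allowed rewards.
; Options spawn as BP_Card actors; on confirm, unchosen ones are destroyed and the pick, or an empty array, is passed on.
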(event Custom|BindToCardConfirm
  (params (CardRewardScreen :type WBP%20Card%20Reward%20Screen%20Object%20Reference))
  (EventDispatchers|BindEventtoOnReturnSelectedCard CardRewardScreen (delegate Custom|ValidateAndTransferSelectedCard)))

(event Custom|ValidateAndTransferSelectedCard
  (params (bSkipped :type Boolean) (Card :type BP%20Card%20Object%20Reference))
  (EventDispatchers|UnbindEventfromOnReturnSelectedCard (stale Custom|BindToCardConfirm CardRewardScreen) (delegate Custom|ValidateAndTransferSelectedCard))
  (for _array_element (Variables|Default|GetCurrentCardOptions)
    (if (!= _array_element Card)
      (if (Utilities|IsValid _array_element)
        (Actor|DestroyActor _array_element))))
  (if (Utilities|IsValid Card)
    (Variables|/Game/ShamanCardGame/Widgets/WBP_CardHand.WBP_CardHand_C|SetbSelectionMode (Variables|/Game/ShamanCardGame/Widgets/WBP_Layout_RLDB.WBP_Layout_RLDB_C|GetWBP_Hand (Variables|/Game/ShamanCardGame/Blueprints/Core/BP_CardPlayer.BP_CardPlayer_C|GetPlayerUI (CallFunction|GetCardPlayerPure))) false)
    (Default|CallOnInputTargetsReceived (Utilities|Array|MakeArray Card))
    (else
      (Default|CallOnInputTargetsReceived (Variables|Default|GetEmptyArray)))))

(fn FindValidTargets
  (params (SpecifiedTargets :type Array%20of%20Actor%20Object%20References) (CardEffect :type F%20Card%20Effect%20Structure) (Card :type BP%20Card%20Object%20Reference) (bPreview :type Boolean))
  (bind _gameplaytags (CallFunction|GetEffectGameplayTags CardEffect))
  (bind _useddata (CallFunction|GetEffectUsedData CardEffect))
  (bind _useddata_2 (CallFunction|GetEffectUsedData CardEffect))
  (if bPreview
    (return false 0)
    (else
      (Utilities|Casting|CastToBP_PileComponentClass (CallFunction|GetEffectTargetComponent CardEffect)
        (:then
          (Utilities|Array|Clear (Variables|Default|GetCurrentCardOptions))
          (if (Utilities|IsValid (.datatable (CallFunction|GetEffectUsedData CardEffect)))
            (if (GameplayTags|HasTag (CallFunction|GetEffectGameplayTags CardEffect) "(TagName=\"Flag.Specific\")" true)
              (bind _returnvalue (Utilities|GetDataTableRow (.datatable _useddata) (.rowname _useddata))
                (:then
                  (LocalVariables|SetLocalCardOptions (Utilities|Array|MakeArray _returnvalue))))
              (else
                (bind _returnvalue_2 (Utilities|GetDataTableRow (.datatable _useddata_2) (.rowname _useddata_2))
                  (:then
                    (LocalVariables|SetLocalRarityWeights (Utilities|Struct|BreakFRarityWeights _returnvalue_2))
                    (bind _allowedcardrewards (Class|BPICardGameInstance|GetAllowedCardRewardsfromInstance(Message) (Game|GetGameInstance)))
                    (bind _randomcards (Default|GetRandomCardsbyTagWeights :self (Variables|/Game/ShamanCardGame/Blueprints/Core/BP_CardPlayer.BP_CardPlayer_C|GetBP_ChanceManagerComponent (CallFunction|GetCardPlayerPure)) :TagWeights (LocalVariables|GetLocalRarityWeights) :PossibleTags (select (GameplayTags|HasTag (CallFunction|GetEffectGameplayTags CardEffect) "(TagName=\"Flag.FilterToAllowed\")") _allowedcardrewards "") :Amount 3))
                    (LocalVariables|SetLocalCardOptions _randomcards))
                  (:RowNotFound
                    (if (GameplayTags|HasTag (CallFunction|GetEffectGameplayTags CardEffect) "(TagName=\"Flag.FilterToAllowed\")") :!label _label
                      (bind _allowedcardrewards_2 (Class|BPICardGameInstance|GetAllowedCardRewardsfromInstance(Message) (Game|GetGameInstance)))
                      (bind _randomcards_2 (Default|GetRandomFilteredCards (Variables|/Game/ShamanCardGame/Blueprints/Core/BP_CardPlayer.BP_CardPlayer_C|GetBP_ChanceManagerComponent (CallFunction|GetCardPlayerPure)) 3 _allowedcardrewards_2 "(GameplayTags=((TagName=\"Rarity\")))" false))
                      (LocalVariables|SetLocalCardOptions _randomcards_2)
                      (else
                        (bind _randomcards_3 (Default|GetTrueRandomCardsOfAnyRarity (Variables|/Game/ShamanCardGame/Blueprints/Core/BP_CardPlayer.BP_CardPlayer_C|GetBP_ChanceManagerComponent (CallFunction|GetCardPlayerPure)) 3))
                        (LocalVariables|SetLocalCardOptions _randomcards_3)))))))
            (else
              (goto _label)))
          (for _array_element (LocalVariables|GetLocalCardOptions)
            (bind _returnvalue_3 (Game|SpawnActorfromClass "/Game/ShamanCardGame/Blueprints/Core/BP_Card.BP_Card_C" (Math|Transform|MakeTransform "0, 0, 0" "0, 0, 0" "1.000000,1.000000,1.000000") "AlwaysSpawn" "OverrideRootScale" (Components|GetOwner Card) _array_element 0))
            (Utilities|Array|Add (Variables|Default|GetCurrentCardOptions) _returnvalue_3))
          (Game|SpawnActorfromClass "/Game/ShamanCardGame/Blueprints/CardActions/BP_Action_CardRewardScreen.BP_Action_CardRewardScreen_C" (Math|Transform|MakeTransform "0, 0, 0" "0, 0, 0" "1.000000,1.000000,1.000000") "AlwaysSpawn" "OverrideRootScale" 0 (Variables|Default|GetCurrentCardOptions) (select (GameplayTags|HasTag _gameplaytags "(TagName=\"Flag.Specific\")" true) "Card Granted" "Choose a Card") (GameplayTags|HasTag _gameplaytags "(TagName=\"Flag.Skippable\")" true) -1.0 0)
          (CallFunction|BindtoCardConfirm (Variables|/Game/ShamanCardGame/Widgets/WBP_Layout_RLDB.WBP_Layout_RLDB_C|GetWBP_CardRewardScreen (Variables|/Game/ShamanCardGame/Blueprints/Core/BP_CardPlayer.BP_CardPlayer_C|GetPlayerUI (CallFunction|GetCardPlayerPure))))
          (return true 0))
        (:CastFailed
          (return false 0))))))