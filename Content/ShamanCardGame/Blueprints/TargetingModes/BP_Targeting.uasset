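; BP_Targeting is the apparent base for card-effect targeting modes in the card game, with a stub FindValidTargets that always reports success.
; Helper functions gather minions by gameplay tag, scanning "Minion"-tagged actors for any exact match on their BP_GameplayTagComponent.
; Others resolve a card's owning minion to its track and opposing track, then return the minions on the opposing side.
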(fn FindValidTargets
  (params (SpecifiedTargets :type Array%20of%20Actor%20Object%20References) (CardEffect :type F%20Card%20Effect%20Structure) (Card :type BP%20Card%20Object%20Reference) (bPreview :type Boolean))
  (return true (Utilities|Array|MakeArray 0)))

(fn FindAllMinionswithMatchingTags
  (params (GameplayTags :type Gameplay%20Tag%20Container%20Structure%20%28by%20ref%29))
  (bind _outactors (Actor|GetAllActorswithTag "Minion"))
  (for _array_element _outactors
    (Utilities|IsValid (Actor|GetComponentbyClass _array_element "/Game/ShamanCardGame/Blueprints/Core/BP_GameplayTagComponent.BP_GameplayTagComponent_C")
      (:Is%20Valid
        (if (GameplayTags|HasAnyTags GameplayTags (Variables|/Game/ShamanCardGame/Blueprints/Core/BP_GameplayTagComponent.BP_GameplayTagComponent_C|GetGameplayTags (Actor|GetComponentbyClass _array_element "/Game/ShamanCardGame/Blueprints/Core/BP_GameplayTagComponent.BP_GameplayTagComponent_C")) true)
          (Utilities|Array|Add (LocalVariables|GetLocalMatchingTargets) _array_element)))))
  (return (LocalVariables|GetLocalMatchingTargets)))

(fn FindMinionTracks
  (params (Card :type BP%20Card%20Object%20Reference))
  (bind _asbp_minion (Utilities|Casting|CastToBP_Minion (Components|GetOwner Card))
    (:then
      (bind _miniontrack (Variables|/Game/ShamanCardGame/Blueprints/Core/BP_Minion.BP_Minion_C|GetMinionTrack _asbp_minion)
        (:then
          (bind _opposingtrack (Variables|/Game/ShamanCardGame/Blueprints/Core/BP_MinionTrack.BP_MinionTrack_C|GetOpposingTrack _miniontrack)
            (:then
              (return _miniontrack _opposingtrack))
            (:else
              (return _miniontrack 0))))
        (:else
          _)))
    (:CastFailed
      _))
  (return 0 0))

(fn GetAllMinionsonOpposingTrack
  (params (Card :type BP%20Card%20Object%20Reference))
  (bind _opposingtrack (CallFunction|FindMinionTracks Card))
  (Utilities|IsValid _opposingtrack
    (:Is%20Valid
      (if (> (Utilities|Array|Length (Variables|/Game/ShamanCardGame/Blueprints/Core/BP_MinionTrack.BP_MinionTrack_C|GetMinions _opposingtrack)) 0)
        (return true (Variables|/Game/ShamanCardGame/Blueprints/Core/BP_MinionTrack.BP_MinionTrack_C|GetMinions _opposingtrack))
        (else
          (return false 0))))
    (:Is%20Not%20Valid
      (return false 0))))