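; Targeting mode for card effects that target cards in the player's hand, filtered by the effect's gameplay tags.
; If matches exceed the effect's value, it queues a selection-mode event and has the hand UI let the player pick that many.
; Otherwise it passes all matches on immediately.
; Confirmed picks return through a temporary binding to the hand widget, and previews never find targets.
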(event Custom|BindToCardConfirm
  (params (Hand :type WBP%20Card%20Hand%20Object%20Reference))
  (bind _output_get (Variables|Default|SetBoundHand Hand))
  (EventDispatchers|BindEventtoReturnSelectedCards _output_get (delegate Custom|ValidateAndTransferSelectedCards)))

(event Custom|ValidateAndTransferSelectedCards
  (params (Cards :type Array%20of%20BP%20Card%20Object%20References))
  (bind _boundhand (Variables|Default|GetBoundHand)
    (:then
      (EventDispatchers|UnbindEventfromReturnSelectedCards _boundhand (delegate Custom|ValidateAndTransferSelectedCards)))
    (:else
      _))
  (Default|CallOnInputTargetsReceived Cards))

(fn FindValidTargets
  (params (SpecifiedTargets :type Array%20of%20Actor%20Object%20References) (CardEffect :type F%20Card%20Effect%20Structure) (Card :type BP%20Card%20Object%20Reference) (bPreview :type Boolean))
  (bind _localvalidcards (LocalVariables|GetLocalValidCards))
  (bind _gameplaytags (CallFunction|GetEffectGameplayTags CardEffect))
  (if bPreview
    (return false 0)
    (else
      (bind _cardplayer (CallFunction|GetCardPlayer))
      (for _array_element (Variables|/Game/ShamanCardGame/Blueprints/Piles/BP_PileComponent.BP_PileComponent_C|GetCards (Actor|GetComponentbyClass _cardplayer "/Game/ShamanCardGame/Blueprints/Piles/BP_PileComponent_Hand.BP_PileComponent_Hand_C"))
        (if (or (== _gameplaytags (Variables|Default|GetEmptyTagContainer)) (GameplayTags|HasAnyTags _gameplaytags (Variables|/Game/ShamanCardGame/Blueprints/Core/BP_GameplayTagComponent.BP_GameplayTagComponent_C|GetGameplayTags (Actor|GetComponentbyClass _array_element "/Game/ShamanCardGame/Blueprints/Core/BP_GameplayTagComponent.BP_GameplayTagComponent_C")) true))
          (Utilities|Array|Add (LocalVariables|GetLocalValidCards) _array_element)))
      (if (> (Utilities|Array|Length (LocalVariables|GetLocalValidCards)) 0)
        (if (> (Utilities|Array|Length (LocalVariables|GetLocalValidCards)) (CallFunction|GetEffectValue CardEffect))
          (CallFunction|QueueEventinGlobalDispatcherHub "(TagName=\"Event.CardSelectionMode\")" Card 0 -1.0)
          (bind _cardplayer_2 (CallFunction|GetCardPlayer))
          (CallFunction|BindtoCardConfirm (Variables|/Game/ShamanCardGame/Widgets/WBP_Layout_RLDB.WBP_Layout_RLDB_C|GetWBP_Hand (Variables|/Game/ShamanCardGame/Blueprints/Core/BP_CardPlayer.BP_CardPlayer_C|GetPlayerUI _cardplayer_2)))
          (Default|EnableSelectionMode (Variables|/Game/ShamanCardGame/Widgets/WBP_Layout_RLDB.WBP_Layout_RLDB_C|GetWBP_Hand (Variables|/Game/ShamanCardGame/Blueprints/Core/BP_CardPlayer.BP_CardPlayer_C|GetPlayerUI _cardplayer_2)) (CallFunction|GetEffectValue CardEffect) (CallFunction|GetEffectGameplayTags CardEffect))
          (return true 0)
          (else
            (CallFunction|ValidateandTransferSelectedCards _localvalidcards)
            (return true _localvalidcards)))
        (else
          (return false (LocalVariables|GetLocalValidCards)))))))