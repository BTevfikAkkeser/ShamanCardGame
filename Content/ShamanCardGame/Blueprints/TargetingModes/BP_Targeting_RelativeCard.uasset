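; BP_Targeting_RelativeCard is a card effect targeting mode that selects the card immediately after the given card in the player's hand.
; FindValidTargets looks up the card's index in the hand pile and returns its next neighbor, failing when the card is absent or last.
; The +1 offset is hardcoded, SpecifiedTargets, CardEffect and Preview are unused, and a debug print outputs the index.
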(fn FindValidTargets
  (params (SpecifiedTargets :type Array%20of%20Actor%20Object%20References) (CardEffect :type F%20Card%20Effect%20Structure) (Card :type BP%20Card%20Object%20Reference) (bPreview :type Boolean))
  (bind _cardplayer (CallFunction|GetCardPlayer))
  (Development|PrintString (Utilities|String|ToString(Integer) (Utilities|Array|FindItem (Variables|/Game/ShamanCardGame/Blueprints/Piles/BP_PileComponent.BP_PileComponent_C|GetCards (Variables|/Game/ShamanCardGame/Blueprints/Core/BP_CardPlayer.BP_CardPlayer_C|GetBP_PileComponent_Hand _cardplayer)) Card)))
  (if (and (>= (Utilities|Array|FindItem (Variables|/Game/ShamanCardGame/Blueprints/Piles/BP_PileComponent.BP_PileComponent_C|GetCards (Variables|/Game/ShamanCardGame/Blueprints/Core/BP_CardPlayer.BP_CardPlayer_C|GetBP_PileComponent_Hand _cardplayer)) Card) 0) (< (Utilities|Array|FindItem (Variables|/Game/ShamanCardGame/Blueprints/Piles/BP_PileComponent.BP_PileComponent_C|GetCards (Variables|/Game/ShamanCardGame/Blueprints/Core/BP_CardPlayer.BP_CardPlayer_C|GetBP_PileComponent_Hand _cardplayer)) Card) (Utilities|Array|LastIndex (Variables|/Game/ShamanCardGame/Blueprints/Piles/BP_PileComponent.BP_PileComponent_C|GetCards (Variables|/Game/ShamanCardGame/Blueprints/Core/BP_CardPlayer.BP_CardPlayer_C|GetBP_PileComponent_Hand _cardplayer)))))
    (bind _cardplayer_2 (CallFunction|GetCardPlayer))
    (return true (Utilities|Array|MakeArray (Utilities|Array|Get(acopy) (Variables|/Game/ShamanCardGame/Blueprints/Piles/BP_PileComponent.BP_PileComponent_C|GetCards (Variables|/Game/ShamanCardGame/Blueprints/Core/BP_CardPlayer.BP_CardPlayer_C|GetBP_PileComponent_Hand _cardplayer_2)) (+ (Utilities|Array|FindItem (Variables|/Game/ShamanCardGame/Blueprints/Piles/BP_PileComponent.BP_PileComponent_C|GetCards (Variables|/Game/ShamanCardGame/Blueprints/Core/BP_CardPlayer.BP_CardPlayer_C|GetBP_PileComponent_Hand _cardplayer_2)) Card) 1))))
    (else
      (return false 0))))