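; Card effect for the card game that grants a status in proportion to matching statuses on the target actor.
; ResolveCardEffect totals StatusValue across the target's BP_Status components that have any gameplay tag exactly matching the effect's GameplayTags.
; It casts TargetComponent to BP_Status and passes it with that total to AddToStatusMessage on the target, returning false if the cast fails.
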(fn ResolveCardEffect
  (params (TargetActor :type Actor%20Object%20Reference))
  (bind _arrayelement (Utilities|Array|ReverseforEachLoop (Actor|GetComponentsByClass TargetActor "/Game/ShamanCardGame/Blueprints/Statuses/BP_Status.BP_Status_C"))
    (:LoopBody
      (if (GameplayTags|HasAnyTags (Variables|/Game/ShamanCardGame/Blueprints/Statuses/BP_Status.BP_Status_C|GetGameplayTags _arrayelement) (Variables|Default|GetGameplayTags) true)
        (LocalVariables|SetValidStatusCount (+ (Variables|/Game/ShamanCardGame/Blueprints/Statuses/BP_Status.BP_Status_C|GetStatusValue _arrayelement) (LocalVariables|GetValidStatusCount)))))
    (:Completed
      (bind _asbp_status (Utilities|Casting|CastToBP_StatusClass (Variables|Default|GetTargetComponent))
        (:then
          (Class|BPICardTarget|AddtoStatus(Message) TargetActor _asbp_status (LocalVariables|GetValidStatusCount) true)
          (return true))
        (:CastFailed
          (return false))))))