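; Card effect that permanently adds or subtracts damage on a target attack card in the shaman card game.
; ResolveCardEffect casts the target to BP_Card and applies EffectValue to its Attack-tagged effects in two passes, covering hand and pile so discarding does not reset it.
; It then fires the ModifyInHand card event and returns true, or false when the target is not a card.
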(fn ResolveCardEffect
  (params (TargetActor :type Actor%20Object%20Reference))
  ;[0 0 0] Changes the damage of an attack card, both in hand and in pile (is not reset when discarded). Required input: Target Actor (Card), Effect Value (Damage to be added/subtracted)
  (bind _asbp_card (Utilities|Casting|CastToBP_Card TargetActor)
    (:then
      (bind _output_get (LocalVariables|SetLocalCard _asbp_card))
      (Default|ModifyCardEffectValues :self _output_get :Modification (Variables|Default|GetEffectValue) :RequiredTags "(GameplayTags=((TagName=\"Effect.Attack\")))")
      (Default|ModifyCardEffectValues :self (LocalVariables|GetLocalCard) :Modification (Variables|Default|GetEffectValue) :Type "NewEnumerator3" :RequiredTags "(GameplayTags=((TagName=\"Effect.Attack\")))")
      (Default|CallLocalEventonCard (LocalVariables|GetLocalCard) "(TagName=\"Event.Card.ModifyInHand\")" "NewEnumerator1")
      (return true))
    (:CastFailed
      (return false))))