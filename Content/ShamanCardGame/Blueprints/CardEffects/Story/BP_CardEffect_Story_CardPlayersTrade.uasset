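; Story card effect that reacts to a traded card by continuing the story encounter with an outcome based on that card's rarity.
; ResolveCardEffect casts the target to BP_Card, switches on its Rarity tag and initializes a non-first encounter screen on the card player.
; Common and Rare share the common encounter, Epic and Legendary share the epic one, and any other rarity gets the trash encounter.
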(fn ResolveCardEffect
  (params (TargetActor :type Actor%20Object%20Reference))
  (bind _asbp_card (Utilities|Casting|CastToBP_Card TargetActor))
  (|SwitchGameplayTag (Variables|/Game/ShamanCardGame/Blueprints/Core/BP_Card.BP_Card_C|GetRarity _asbp_card)
    (:Default
      (Default|InitializeStoryEncounter (CallFunction|GetCardPlayerPure) (Variables|Default|GetTrashEncounter) false))
    (:Rarity.Common
      (Default|InitializeStoryEncounter (CallFunction|GetCardPlayerPure) (Variables|Default|GetCommonEncounter) false :!label _label))
    (:Rarity.Rare
      (goto _label))
    (:Rarity.Epic
      (Default|InitializeStoryEncounter (CallFunction|GetCardPlayerPure) (Variables|Default|GetEpicEncounter) false :!label _label_2))
    (:Rarity.Legendary
      (goto _label_2)))
  (return true))