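; Story card effect that modifies the persistent health of heroes from the game instance.
; On resolve it fetches the persistent heroes through a game instance message and loops over each one.
; Each hero's starting health status plus the effect value is clamped between zero and its health status limit, then sent back by unique ID as the new persistent health.
; The target actor is ignored.
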(fn ResolveCardEffect
  (params (TargetActor :type Actor%20Object%20Reference))
  (bind _persistentheroes (Class|BPICardGameInstance|GetPersistentHeroesfromInstance(Message) (Game|GetGameInstance)))
  (for _array_element _persistentheroes
    (Class|BPICardGameInstance|UpdateHeroPersistentHealth(Message) (Game|GetGameInstance) (.UniqueID (Utilities|Struct|BreakFMinion _array_element)) (Math|Integer|Max(Integer) (Math|Integer|Min(Integer) (+ (.Value (Utilities|Map|Find (.StartingStatuses (Utilities|Struct|BreakFMinion _array_element)) "/Game/ShamanCardGame/Blueprints/Statuses/BP_Status_Health.BP_Status_Health_C")) (Variables|Default|GetEffectValue)) (.Value (Utilities|Map|Find (.StatusLimits (Utilities|Struct|BreakFMinion _array_element)) "/Game/ShamanCardGame/Blueprints/Statuses/BP_Status_Health.BP_Status_Health_C"))))))
  (return true))