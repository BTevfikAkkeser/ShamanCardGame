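; Story card effect for the Nokken altar that upgrades a target card, tinting its frame green and appending "+" to its name.
; Attack and Defense cards pass their current effect value back in as the modification, apparently doubling it; other types get their Mana stat-cost rule set instead.
; All edits target one card data set, which is then copied over to the other.
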(fn ResolveCardEffect
  (params (TargetActor :type Actor%20Object%20Reference))
  (bind _asbp_card (Utilities|Casting|CastToBP_Card TargetActor))
  (Default|SetCardFrameTint _asbp_card "NewEnumerator1" (Utilities|Struct|MakeSlateColor "(R=0.488050,G=0.656250,B=0.453003,A=1.000000)" "UseColor_Specified"))
  (Default|SetCardName _asbp_card "NewEnumerator1" (Utilities|Text|ToText(String) (Utilities|String|Append (Utilities|String|ToString(Text) (Default|GetCardName _asbp_card "NewEnumerator1")) " +")))
  (|SwitchGameplayTag (Variables|/Game/ShamanCardGame/Blueprints/Core/BP_Card.BP_Card_C|GetType _asbp_card)
    (:Default
      (Default|SetUseRuleCost _asbp_card "/Game/ShamanCardGame/Blueprints/CardUseRules/BP_UseRule_StatCost.BP_UseRule_StatCost_C" "/Game/ShamanCardGame/Blueprints/Statuses/BP_Status_Mana.BP_Status_Mana_C" 0 "NewEnumerator1" false))
    (:Effect.Attack
      (bind (_bsuccess _effectvalue) (Default|GetCardEffectValue :self _asbp_card :PossibleTags (GameplayTags|MakeGameplayTagContainerfromTag (Variables|/Game/ShamanCardGame/Blueprints/Core/BP_Card.BP_Card_C|GetType _asbp_card)) :Type "NewEnumerator1" :!label _label))
      (if _bsuccess
        (Default|ModifyCardEffectValues _asbp_card _effectvalue "NewEnumerator1" (GameplayTags|MakeGameplayTagContainerfromTag (Variables|/Game/ShamanCardGame/Blueprints/Core/BP_Card.BP_Card_C|GetType _asbp_card)))))
    (:Effect.Defense
      (goto _label)))
  (Default|SetCardDatafromOtherData _asbp_card "NewEnumerator1" "NewEnumerator0")
  (return true))