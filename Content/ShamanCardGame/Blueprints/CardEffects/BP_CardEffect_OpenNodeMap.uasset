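; BP_CardEffect_OpenNodeMap is a card effect that travels to a node map level when resolved.
; An empty Identifier opens the current node map stored in the game instance.
; Otherwise it records Identifier as the current node map through a game instance message and opens that level by name.
; TargetActor is unused, and both paths report success.
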(fn ResolveCardEffect
  (params (TargetActor :type Actor%20Object%20Reference))
  (if (Utilities|Array|IsEmpty (Variables|Default|GetIdentifier))
    (bind _currentnodemap (Class|BPICardGameInstance|GetCurrentNodeMapfromInstance(Message) (Game|GetGameInstance)))
    (Game|OpenLevel(byName) (Utilities|String|StringToName _currentnodemap))
    (return true)
    (else
      (Class|BPICardGameInstance|ChangeNodeMapinInstance(Message) (Game|GetGameInstance) (Variables|Default|GetIdentifier))
      (Game|OpenLevel(byName) (Utilities|String|StringToName (Variables|Default|GetIdentifier)))
      (return true))))