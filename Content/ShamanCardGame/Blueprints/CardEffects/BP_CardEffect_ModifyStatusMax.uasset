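; BP_CardEffect_ModifyStatusMax is a card effect that changes the maximum value of a status on the target actor.
; ResolveCardEffect looks up the status component by the TargetComponent class and, if it is Maxable, adds EffectValue to its MaxValue, clamped at zero, through SetStatusMax.
; It returns true when the maximum is set, and false if the component is not a BP_Status, is missing or is not Maxable.
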(fn ResolveCardEffect
  (params (TargetActor :type Actor%20Object%20Reference))
  (bind _targetcomponent (Variables|Default|GetTargetComponent))
  (bind _returnvalue (Actor|GetComponentbyClass TargetActor _targetcomponent))
  (bind _asbp_status (Utilities|Casting|CastToBP_Status _returnvalue))
  (Utilities|Casting|CastToBP_StatusClass (Variables|Default|GetTargetComponent)
    (:then
      (if (Utilities|IsValid _returnvalue)
        (if (Variables|/Game/ShamanCardGame/Blueprints/Statuses/BP_Status.BP_Status_C|GetbMaxable _asbp_status)
          (Default|SetStatusMax _asbp_status (Math|Integer|Max(Integer) (+ (Variables|/Game/ShamanCardGame/Blueprints/Statuses/BP_Status.BP_Status_C|GetMaxValue _asbp_status) (Variables|Default|GetEffectValue))))
          (return true)
          (else
            _)))
      (return false))
    (:CastFailed
      (return false))))