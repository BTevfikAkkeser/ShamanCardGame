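; Card effect that generates random cards of any rarity and adds them to one of the card player's piles, defaulting to the hand.
; The player's chance manager picks the card data, with the effect value setting the count.
; Each pick spawns as a new card actor and is offered to the pile component matching the target class.
; Cards that are added successfully fire the card Generate event.
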(fn ResolveCardEffect
  (params (TargetActor :type Actor%20Object%20Reference))
  (bind _asbp_pile_component (Utilities|Casting|CastToBP_PileComponentClass (Variables|Default|GetTargetComponent)) ; If no pile is specified, adds to hand
    (:then
      (LocalVariables|SetLocalTargetPileClass _asbp_pile_component))
    (:CastFailed
      (LocalVariables|SetLocalTargetPileClass "/Game/ShamanCardGame/Blueprints/Piles/BP_PileComponent_Hand.BP_PileComponent_Hand_C")))
  (bind _cardplayer (CallFunction|GetCardPlayer))
  (bind _randomcards (Default|GetTrueRandomCardsOfAnyRarity (Variables|/Game/ShamanCardGame/Blueprints/Core/BP_CardPlayer.BP_CardPlayer_C|GetBP_ChanceManagerComponent _cardplayer) (Variables|Default|GetEffectValue)))
  (for _array_element _randomcards
    (bind _returnvalue (Game|SpawnActorfromClass "/Game/ShamanCardGame/Blueprints/Core/BP_Card.BP_Card_C" (Math|Transform|MakeTransform "0, 0, 0" "0, 0, 0" "1.000000,1.000000,1.000000") "AlwaysSpawn" "OverrideRootScale" (Components|GetOwner (Variables|Default|GetParentCard)) _array_element 0))
    (Utilities|Array|Add (LocalVariables|GetLocalCards) _returnvalue)
    (bind _bsuccess (Class|BPIPile|AttemptAddExistingCard(Message) (Actor|GetComponentbyClass (CallFunction|GetCardPlayerPure) (LocalVariables|GetLocalTargetPileClass)) _returnvalue))
    (if _bsuccess
      (Default|CallLocalEventonCard _returnvalue "(TagName=\"Event.Card.Generate\")" "NewEnumerator2")))
  (return true))