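; Card effect for the Big Deck Energy card that grants a status to its target based on draw pile size.
; ResolveCardEffect casts the target component to BP_Status, then divides the card player's draw pile count by the effect value and rounds down.
; It sends that amount to the target as an add-status message with itself as payload, returning false if the cast fails.
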(fn ResolveCardEffect
  (params (TargetActor :type Actor%20Object%20Reference))
  ;[0 0 0] Used for the Big Deck Energy card. Adds 1 of the specified status to the target for each [status value] number of cards in the Draw Pile
  (bind _asbp_status (Utilities|Casting|CastToBP_StatusClass (Variables|Default|GetTargetComponent))
    (:then
      (bind _cardplayer (CallFunction|GetCardPlayer))
      (Class|BPICardTarget|AddtoStatus(Message) TargetActor _asbp_status (Math|Float|Floor (/ (Math|Conversions|ToFloat(Integer) (Utilities|Array|Length (Variables|/Game/ShamanCardGame/Blueprints/Piles/BP_PileComponent.BP_PileComponent_C|GetCards (Variables|/Game/ShamanCardGame/Blueprints/Core/BP_CardPlayer.BP_CardPlayer_C|GetBP_PileComponent_Draw _cardplayer)))) (Math|Conversions|ToFloat(Integer) (Variables|Default|GetEffectValue)))) true self)
      (return true))
    (:CastFailed
      (return false))))