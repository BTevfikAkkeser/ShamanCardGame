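; Fear status for the card game that halves the Attack value of its owner's attack cards.
; RunEvent applies the cut on card draw, generate and modify-in-hand events, and removes one stack when the owner's turn starts.
; Adding stacks fires a modify-in-hand event on each card in the card player's hand so held cards can update.
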(event EventBeginPlay
  (CallFunction|BindMultipleEventstoGlobalDispatcherHub self "(GameplayTags=((TagName=\"Event.Card.Draw\"),(TagName=\"Event.Card.Generate\"),(TagName=\"Event.Card.ModifyInHand\")))")
  (Default|BindEventtoHub (.ReturnValue (CallFunction|GetOwnersDispatcherHub)) self "(TagName=\"Event.TurnStart\")")
  (|CallParentFunction))

(event EventRunEvent
  (params (EventTag :type Gameplay%20Tag%20Structure) (CallingObject :type Object%20Object%20Reference%20%28by%20ref%29) (bGlobal :type Boolean) (Payload :type Object%20Object%20Reference%20%28by%20ref%29) (CallTags :type Gameplay%20Tag%20Container%20Structure%20%28by%20ref%29))
  (|SwitchGameplayTag EventTag
    (:Event.Card.Draw
      (bind _asbp_card (Utilities|Casting|CastToBP_Card CallingObject :!label _label))
      (if (== (Components|GetOwner _asbp_card) (Components|GetOwner))
        (if (== (Variables|/Game/ShamanCardGame/Blueprints/Core/BP_Card.BP_Card_C|GetType _asbp_card) "(TagName=\"Effect.Attack\")")
          (bind (_bsuccess _effectvalue) (Default|GetCardEffectValue :self _asbp_card :RequiredTags "(GameplayTags=((TagName=\"Effect.Attack\")))"))
          (if _bsuccess
            (Default|ModifyCardEffectValues :self _asbp_card :Modification (* (/ _effectvalue 2) -1) :RequiredTags "(GameplayTags=((TagName=\"Effect.Attack\")))")))))
    (:Event.Card.Generate
      (goto _label))
    (:Event.Card.ModifyInHand
      (goto _label))
    (:Event.TurnStart
      (if (== CallingObject (Components|GetOwner))
        (CallFunction|SubtractStatusValue 1 false false)))))

(fn AddStatusValue
  (params (Amount :type Integer) (bShowSplashNumber :type Boolean) (bShowSplashIcon :type Boolean) (bRefreshAppearance :type Boolean) (Payload :type Object%20Object%20Reference))
  (bind _newvalue (|CallParentFunction Amount bShowSplashNumber bShowSplashIcon false 0))
  (bind _cardplayer (CallFunction|GetCardPlayer))
  (for _array_element (Variables|/Game/ShamanCardGame/Blueprints/Piles/BP_PileComponent.BP_PileComponent_C|GetCards (Actor|GetComponentbyClass _cardplayer "/Game/ShamanCardGame/Blueprints/Piles/BP_PileComponent_Hand.BP_PileComponent_Hand_C"))
    (Default|CallLocalEventonCard _array_element "(TagName=\"Event.Card.ModifyInHand\")" "NewEnumerator1"))
  (return _newvalue))