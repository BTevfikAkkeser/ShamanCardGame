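; BP_Status_HandSizeArmor is a card game status that turns the number of cards held in hand into armor.
; On BeginPlay it registers with the card player's local dispatcher hub for the turn end event.
; When that event runs, it counts the cards in the player's hand pile and, if any, sends its owner an add-status message for that amount of BP_Status_Armor.
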(event EventBeginPlay
  (|CallParentFunction)
  (bind _cardplayer (CallFunction|GetCardPlayer))
  (bind _bp_dispatcherhubcomponent_local (Variables|/Game/ShamanCardGame/Blueprints/Core/BP_CardPlayer.BP_CardPlayer_C|GetBP_DispatcherHubComponent_Local _cardplayer)
    (:then
      (Default|BindEventtoHub _bp_dispatcherhubcomponent_local self "(TagName=\"Event.TurnEnd\")"))
    (:else)))

(event EventRunEvent
  (params (EventTag :type Gameplay%20Tag%20Structure) (CallingObject :type Object%20Object%20Reference%20%28by%20ref%29) (bGlobal :type Boolean) (Payload :type Object%20Object%20Reference%20%28by%20ref%29) (CallTags :type Gameplay%20Tag%20Container%20Structure%20%28by%20ref%29))
  (|SwitchGameplayTag EventTag
    (:Event.TurnEnd
      (bind _cardplayer (CallFunction|GetCardPlayer))
      (if (> (Utilities|Array|Length (Variables|/Game/ShamanCardGame/Blueprints/Piles/BP_PileComponent.BP_PileComponent_C|GetCards (Actor|GetComponentbyClass _cardplayer "/Game/ShamanCardGame/Blueprints/Piles/BP_PileComponent_Hand.BP_PileComponent_Hand_C"))) 0)
        (Class|BPICardTarget|AddtoStatus(Message) (Components|GetOwner) "/Game/ShamanCardGame/Blueprints/Statuses/BP_Status_Armor.BP_Status_Armor_C" (Utilities|Array|Length (Variables|/Game/ShamanCardGame/Blueprints/Piles/BP_PileComponent.BP_PileComponent_C|GetCards (Actor|GetComponentbyClass _cardplayer "/Game/ShamanCardGame/Blueprints/Piles/BP_PileComponent_Hand.BP_PileComponent_Hand_C"))) true)))))