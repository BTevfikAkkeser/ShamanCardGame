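; BP_Status_Barrier is a card game status that shields its owning Minion from incoming damage.
; On BeginPlay it binds itself to the owner's dispatcher hub for the Event.PreTakeDamage tag.
; When RunEvent fires, it casts the calling object to BP_Status, zeroes any negative IncomingStatusChange and spends one point of its own value.
; Damage is intercepted by editing the pending change on the calling status.
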(event EventBeginPlay
  (|CallParentFunction)
  (Default|BindEventtoHub (.ReturnValue (CallFunction|GetOwnersDispatcherHub)) self "(TagName=\"Event.PreTakeDamage\")"))

(event EventRunEvent
  (params (EventTag :type Gameplay%20Tag%20Structure) (CallingObject :type Object%20Object%20Reference%20%28by%20ref%29) (bGlobal :type Boolean) (Payload :type Object%20Object%20Reference%20%28by%20ref%29) (CallTags :type Gameplay%20Tag%20Container%20Structure%20%28by%20ref%29))
  ;[0 0 0] Negates damage from an incoming attack on the owning Minion and reduces the Barrier's effect value by 1
  (|SwitchGameplayTag EventTag
    (:Event.PreTakeDamage
      (bind _asbp_status (Utilities|Casting|CastToBP_Status CallingObject))
      (if (< (Variables|/Game/ShamanCardGame/Blueprints/Statuses/BP_Status.BP_Status_C|GetIncomingStatusChange _asbp_status) 0)
        (Variables|/Game/ShamanCardGame/Blueprints/Statuses/BP_Status.BP_Status_C|SetIncomingStatusChange _asbp_status 0)
        (CallFunction|SubtractStatusValue 1 false false)))))