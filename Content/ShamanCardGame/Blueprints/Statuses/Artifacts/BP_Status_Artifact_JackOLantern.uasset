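; Jack O'Lantern artifact status for the card game that inflicts Fear on enemy minions taking a big enough hit.
; On pre-damage events from the global dispatcher hub, it caches the health status of an enemy minion whose incoming change meets ActivationThreshold.
; The matching post-damage event adds StatusValue Fear to that minion.
; BeginPlay here binds only the pre-damage event, though both are handled.
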(event EventBeginPlay
  (|CallParentFunction)
  (CallFunction|BindMultipleEventstoGlobalDispatcherHub self "(GameplayTags=((TagName=\"Event.PreTakeDamage\"),(TagName=\"Event.PostTakeDamage\")))"))

(event EventRunEvent
  (params (EventTag :type Gameplay%20Tag%20Structure) (CallingObject :type Object%20Object%20Reference%20%28by%20ref%29) (bGlobal :type Boolean) (Payload :type Object%20Object%20Reference%20%28by%20ref%29) (CallTags :type Gameplay%20Tag%20Container%20Structure%20%28by%20ref%29))
  (Utilities|IsValid CallingObject
    (:Is%20Valid
      (|SwitchGameplayTag EventTag
        (:Event.PreTakeDamage
          (Variables|Default|SetAffectedHealthComponent 0)
          (bind _asbp_status_health (Utilities|Casting|CastToBP_Status_Health CallingObject))
          (if (>= (Math|Integer|Absolute(Integer) (Variables|/Game/ShamanCardGame/Blueprints/Statuses/BP_Status.BP_Status_C|GetIncomingStatusChange _asbp_status_health)) (Variables|Default|GetActivationThreshold))
            (bind _asbp_minion (Utilities|Casting|CastToBP_Minion (Components|GetOwner _asbp_status_health)))
            (if (GameplayTags|HasTag (Default|GetGameplayTags _asbp_minion) "(TagName=\"Target.Enemy\")" true)
              (Variables|Default|SetAffectedHealthComponent _asbp_status_health))))
        (:Event.PostTakeDamage
          (if (== CallingObject (Variables|Default|GetAffectedHealthComponent))
            (Class|BPICardTarget|AddtoStatus(Message) (Components|GetOwner (Variables|Default|GetAffectedHealthComponent)) "/Game/ShamanCardGame/Blueprints/Statuses/BP_Status_Fear.BP_Status_Fear_C" (Variables|Default|GetStatusValue) true)))))))