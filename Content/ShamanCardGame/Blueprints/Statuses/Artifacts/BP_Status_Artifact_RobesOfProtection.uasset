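; Artifact status for the Robes of Protection, which grants Armor to heroes while the player's draw pile is large enough.
; On BeginPlay it binds to its owner's dispatcher hub for the turn start event.
; When the event runs, it compares the draw pile's card count to EffectCutoff, then adds StatusValue Armor to every minion in the level tagged as a hero.
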(event EventBeginPlay
  (bind (_bvalid _returnvalue) (CallFunction|GetOwnersDispatcherHub))
  (|CallParentFunction)
  (if _bvalid
    (Default|BindEventtoHub _returnvalue self "(TagName=\"Event.TurnStart\")")))

(event EventRunEvent
  (params (EventTag :type Gameplay%20Tag%20Structure) (CallingObject :type Object%20Object%20Reference%20%28by%20ref%29) (bGlobal :type Boolean) (Payload :type Object%20Object%20Reference%20%28by%20ref%29) (CallTags :type Gameplay%20Tag%20Container%20Structure%20%28by%20ref%29))
  (|SwitchGameplayTag EventTag
    (:Event.TurnStart
      (if (>= (Utilities|Array|Length (Variables|/Game/ShamanCardGame/Blueprints/Piles/BP_PileComponent.BP_PileComponent_C|GetCards (Actor|GetComponentbyClass (CallFunction|GetCardPlayerPure) "/Game/ShamanCardGame/Blueprints/Piles/BP_PileComponent_Draw.BP_PileComponent_Draw_C"))) (Variables|Default|GetEffectCutoff))
        (bind _outactors (Actor|GetAllActorsOfClass "/Game/ShamanCardGame/Blueprints/Core/BP_Minion.BP_Minion_C"))
        (for _array_element _outactors
          (if (GameplayTags|HasTag (Default|GetGameplayTags _array_element) "(TagName=\"Target.Hero\")" true)
            (Default|AddtoStatus _array_element "/Game/ShamanCardGame/Blueprints/Statuses/BP_Status_Armor.BP_Status_Armor_C" (Variables|Default|GetStatusValue) true)))))))