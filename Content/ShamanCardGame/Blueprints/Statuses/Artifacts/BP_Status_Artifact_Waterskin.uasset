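; Waterskin artifact status for the card game that grants the card player mana the first time a card is exhausted each turn.
; On BeginPlay it registers with the global dispatcher hub for card exhaust and turn start events.
; A DoOnce gate lets only the first exhaust add the artifact's status value to the player's Mana status, and turn start resets the gate.
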(event EventBeginPlay
  (|CallParentFunction)
  (CallFunction|BindEventtoGlobalDispatcherHub self "(TagName=\"Event.Card.Exhaust\")")
  (CallFunction|BindEventtoGlobalDispatcherHub self "(TagName=\"Event.TurnStart\")"))

(event EventRunEvent
  (params (EventTag :type Gameplay%20Tag%20Structure) (CallingObject :type Object%20Object%20Reference%20%28by%20ref%29) (bGlobal :type Boolean) (Payload :type Object%20Object%20Reference%20%28by%20ref%29) (CallTags :type Gameplay%20Tag%20Container%20Structure%20%28by%20ref%29))
  (|SwitchGameplayTag EventTag
    (:Event.Card.Exhaust
      (Utilities|FlowControl|DoOnce false :!label _label
        (:Completed
          (Default|AddStatusValue (Actor|GetComponentbyClass (CallFunction|GetCardPlayerPure) "/Game/ShamanCardGame/Blueprints/Statuses/BP_Status_Mana.BP_Status_Mana_C") (Variables|Default|GetStatusValue) false false false))))
    (:Event.TurnStart
      (goto _label Reset))))