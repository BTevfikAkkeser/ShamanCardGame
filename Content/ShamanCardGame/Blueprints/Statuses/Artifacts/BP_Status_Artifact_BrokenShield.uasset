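; Broken Shield artifact status for the card game that grants armor in response to the post-attack event.
; On BeginPlay it retries with a zero delay until the main hero is available, then binds to Event.PostAttack on that hero's local dispatcher hub.
; When the event runs, it adds BP_Status_Armor equal to StatusValue to the owner of the calling component's owner through AddToStatusMessage.
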(event EventBeginPlay
  (|CallParentFunction)
  (bind (_bsuccess _mainhero) (Class|BPICardGameInstance|GetMainHero(Message) (Game|GetGameInstance) :!label _label))
  (if _bsuccess
    (Default|BindEventtoHub (Actor|GetComponentbyClass _mainhero "/Game/ShamanCardGame/Blueprints/Core/BP_DispatcherHubComponent_Local.BP_DispatcherHubComponent_Local_C") self "(TagName=\"Event.PostAttack\")")
    (else
      (Utilities|FlowControl|Delay 0.0)
      (goto _label))))

(event EventRunEvent
  (params (EventTag :type Gameplay%20Tag%20Structure) (CallingObject :type Object%20Object%20Reference%20%28by%20ref%29) (bGlobal :type Boolean) (Payload :type Object%20Object%20Reference%20%28by%20ref%29) (CallTags :type Gameplay%20Tag%20Container%20Structure%20%28by%20ref%29))
  (|SwitchGameplayTag EventTag
    (:Event.PostAttack
      (bind _asactor_component (Utilities|Casting|CastToActorComponent CallingObject))
      (Class|BPICardTarget|AddtoStatus(Message) (Components|GetOwner (Components|GetOwner _asactor_component)) "/Game/ShamanCardGame/Blueprints/Statuses/BP_Status_Armor.BP_Status_Armor_C" (Variables|Default|GetStatusValue) true))))