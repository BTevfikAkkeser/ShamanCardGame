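; Card status that makes its owning card's mana cost drop further each time a card-play event fires while it sits in the hand.
; It listens for global PrePlay and the card's local ExitHand, growing a running reduction by the status value and resetting it outside the hand.
; PrePlay and in-hand modify events recompute the cost from two pile-specific values, never raising it or going below zero, then broadcast the change.
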(event EventBeginPlay
  (|CallParentFunction)
  (CallFunction|BindMultipleEventstoGlobalDispatcherHub self "(GameplayTags=((TagName=\"Event.Card.PrePlay\"),(TagName=\"Event.Card.ModifyInHand\"),(TagName=\"Event.TurnStart\")))")
  (bind _asbp_card (Utilities|Casting|CastToBP_Card (Components|GetOwner)))
  (bind _output_get (Variables|Default|SetOwningCard _asbp_card))
  (Default|BindLocalCardEvents _output_get self "(GameplayTags=((TagName=\"Event.Card.ExitHand\")))"))

(event EventRunEvent
  (params (EventTag :type Gameplay%20Tag%20Structure) (CallingObject :type Object%20Object%20Reference%20%28by%20ref%29) (bGlobal :type Boolean) (Payload :type Object%20Object%20Reference%20%28by%20ref%29) (CallTags :type Gameplay%20Tag%20Container%20Structure%20%28by%20ref%29))
  (if (Utilities|Array|ContainsItem (Variables|/Game/ShamanCardGame/Blueprints/Piles/BP_PileComponent.BP_PileComponent_C|GetCards (Actor|GetComponentbyClass (CallFunction|GetCardPlayerPure) "/Game/ShamanCardGame/Blueprints/Piles/BP_PileComponent_Hand.BP_PileComponent_Hand_C")) (.AsBP%20Card (Utilities|Casting|CastToBP_Card (Components|GetOwner))))
    (|SwitchGameplayTag EventTag
      (:Event.Card.PrePlay
        (Variables|Default|SetCurrentModification (+ (Variables|Default|GetCurrentModification) (Variables|Default|GetStatusValue)))
        (bind (_bvalid _statuscost) (Default|GetStatusCostValuefromUseRules (Variables|Default|GetOwningCard) "NewEnumerator1" "/Game/ShamanCardGame/Blueprints/Statuses/BP_Status_Mana.BP_Status_Mana_C" :!label _label))
        (if _bvalid
          (bind _statuscost_2 (Default|GetStatusCostValuefromUseRules (Variables|Default|GetOwningCard) "NewEnumerator0" "/Game/ShamanCardGame/Blueprints/Statuses/BP_Status_Mana.BP_Status_Mana_C"))
          (bind _bsuccess (Default|SetUseRuleCost (.AsBP%20Card (Utilities|Casting|CastToBP_Card (Components|GetOwner))) "/Game/ShamanCardGame/Blueprints/CardUseRules/BP_UseRule_StatCost.BP_UseRule_StatCost_C" "/Game/ShamanCardGame/Blueprints/Statuses/BP_Status_Mana.BP_Status_Mana_C" (Math|Integer|Max(Integer) (Math|Integer|Min(Integer) _statuscost_2 (- _statuscost (Variables|Default|GetCurrentModification)))) "NewEnumerator0" false))
          (if _bsuccess
            (Default|CallOnThisCardModified (.AsBP%20Card (Utilities|Casting|CastToBP_Card (Components|GetOwner)))))))
      (:Event.Card.ModifyInHand
        (goto _label))
      (:Event.Card.ExitHand
        (Variables|Default|SetCurrentModification 0)))
    (else
      (|SwitchGameplayTag EventTag
        (:Event.TurnStart
          (Variables|Default|SetCurrentModification 0))))))