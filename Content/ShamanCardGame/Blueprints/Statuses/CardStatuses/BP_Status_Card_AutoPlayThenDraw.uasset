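; Card status that makes its owning card play itself when a card draw event fires, then draws for the player.
; On BeginPlay it binds to the Event.Card.Draw tag on the owner's dispatcher hub.
; RunEvent queues a global AutoPlay event and uses the card untargeted, skipping playability checks and consequences.
; Queued delays pace the sequence before the player's hand pile component attempts a draw.
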(event EventBeginPlay
  (|CallParentFunction)
  (Default|BindEventtoHub (.ReturnValue (CallFunction|GetOwnersDispatcherHub)) self "(TagName=\"Event.Card.Draw\")"))

(event EventRunEvent
  (params (EventTag :type Gameplay%20Tag%20Structure) (CallingObject :type Object%20Object%20Reference%20%28by%20ref%29) (bGlobal :type Boolean) (Payload :type Object%20Object%20Reference%20%28by%20ref%29) (CallTags :type Gameplay%20Tag%20Container%20Structure%20%28by%20ref%29))
  (bind _asbp_card (Utilities|Casting|CastToBP_Card (Components|GetOwner)))
  (CallFunction|QueueDelay 0.4)
  (CallFunction|QueueEventinGlobalDispatcherHub "(TagName=\"Event.Action.AutoPlay\")" (Components|GetOwner) 0 1.0)
  (Default|AttemptUseCardUntargeted _asbp_card true true true)
  (CallFunction|QueueDelay 1.0)
  (Default|AttemptDraw (Variables|/Game/ShamanCardGame/Blueprints/Core/BP_CardPlayer.BP_CardPlayer_C|GetBP_PileComponent_Hand (CallFunction|GetCardPlayerPure))))