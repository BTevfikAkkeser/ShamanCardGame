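; Twin Strike status for the card game, which makes its owner's Attack cards repeat when played.
; It binds to the global dispatcher hub's Event.Card.PrePlay event on BeginPlay and filters for cards with the same owner and an exact Effect.Attack tag.
; While the status value is positive, it multiplies the card's total plays by that value plus one, stacking with existing repetitions, then calls SetStatusValue with default input.
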(event EventBeginPlay
  (|CallParentFunction)
  (CallFunction|BindEventtoGlobalDispatcherHub self "(TagName=\"Event.Card.PrePlay\")"))

(event EventRunEvent
  (params (EventTag :type Gameplay%20Tag%20Structure) (CallingObject :type Object%20Object%20Reference%20%28by%20ref%29) (bGlobal :type Boolean) (Payload :type Object%20Object%20Reference%20%28by%20ref%29) (CallTags :type Gameplay%20Tag%20Container%20Structure%20%28by%20ref%29))
  (|SwitchGameplayTag EventTag
    (:Event.Card.PrePlay
      (bind _asbp_card (Utilities|Casting|CastToBP_Card CallingObject))
      (Variables|Default|SetAffectedCard _asbp_card)
      (if (== (Components|GetOwner _asbp_card) (Components|GetOwner))
        (if (GameplayTags|HasTag (Default|GetGameplayTags (Variables|Default|GetAffectedCard)) "(TagName=\"Effect.Attack\")" true)
          (if (> (Variables|Default|GetStatusValue) 0)
            (Default|SetCardRepetitions (Variables|Default|GetAffectedCard) "NewEnumerator0" (- (* (+ (Default|GetCardRepetitions (Variables|Default|GetAffectedCard) "NewEnumerator0") 1) (+ (Variables|Default|GetStatusValue) 1)) 1))
            (CallFunction|SetStatusValue 0 false false)))))))