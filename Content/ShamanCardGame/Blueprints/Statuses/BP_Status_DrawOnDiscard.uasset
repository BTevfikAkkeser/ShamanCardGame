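; A status effect for the card game that draws cards for its owner when cards are discarded.
; On BeginPlay it binds itself to the global dispatcher hub for the card discard event.
; When that event runs with the Active flag, it makes the card player's hand pile attempt draws in a loop driven by the status value.
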(event EventBeginPlay
  (|CallParentFunction)
  (CallFunction|BindEventtoGlobalDispatcherHub self "(TagName=\"Event.Card.Discard\")"))

(event EventRunEvent
  (params (EventTag :type Gameplay%20Tag%20Structure) (CallingObject :type Object%20Object%20Reference%20%28by%20ref%29) (bGlobal :type Boolean) (Payload :type Object%20Object%20Reference%20%28by%20ref%29) (CallTags :type Gameplay%20Tag%20Container%20Structure%20%28by%20ref%29))
  (|SwitchGameplayTag EventTag
    (:Event.Card.Discard
      (if (GameplayTags|HasTag CallTags "(TagName=\"Flag.Active\")" true)
        (bind _cardplayer (CallFunction|GetCardPlayer))
        (for _index (range 0 (Math|Integer|Max(Integer) (- (Variables|Default|GetStatusValue) 1)))
          (Default|AttemptDraw (Variables|/Game/ShamanCardGame/Blueprints/Core/BP_CardPlayer.BP_CardPlayer_C|GetBP_PileComponent_Hand _cardplayer)))))))