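; Minion status that plays cards from the owner's AttackPattern component and displays the upcoming one as an intent icon.
; On the owner's turn start it uses the stored card, then fetches the next from the component, which decides selection.
; It copies that card's portrait, tint, tooltips and attack value with repetitions, queuing a ModifyStatus action to refresh the display.
; Post-modify-status events reset the card's modifications and redisplay only if something changed.
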(event EventBeginPlay
  (bind _returnvalue (Components|GetOwner))
  (bind _returnvalue_2 (Actor|GetComponentbyClass _returnvalue "/Game/ShamanCardGame/Blueprints/Core/BP_AttackPatternComponent.BP_AttackPatternComponent_C"))
  (Utilities|IsValid _returnvalue_2
    (:Is%20Valid
      (Variables|Default|SetAttackPatternRef _returnvalue_2)
      (|CallParentFunction)
      (Default|BindMultipleEventstoHub (.ReturnValue (CallFunction|GetOwnersDispatcherHub)) self "(GameplayTags=((TagName=\"Event.TurnStart\"),(TagName=\"Event.PostModifyStatus\")))")
      (bind _card (Default|GetNextCard (Variables|Default|GetAttackPatternRef)))
      (Variables|Default|SetNextCard _card))))

(event EventRunEvent
  (params (EventTag :type Gameplay%20Tag%20Structure) (CallingObject :type Object%20Object%20Reference%20%28by%20ref%29) (bGlobal :type Boolean) (Payload :type Object%20Object%20Reference%20%28by%20ref%29) (CallTags :type Gameplay%20Tag%20Container%20Structure%20%28by%20ref%29))
  ;[0 0 0] Controls a Minion selecting, displaying and executing a card to use from its AttackPattern component. Which specific card is selected is determined by the AttackPattern component
  (bind _output_get (Variables|Default|SetCurrentEventTag EventTag))
  (|SwitchGameplayTag _output_get
    (:Event.TurnStart
      (if (and (== CallingObject (Components|GetOwner)) (not bGlobal))
        (bind _nextcard (Variables|Default|GetNextCard)
          (:then
            (Default|AttemptUseCard _nextcard (Variables|Default|GetEmptyArray) false false false)
            (bind _attackpatternref (Variables|Default|GetAttackPatternRef)
              (:then
                (bind _card (Default|GetNextCard _attackpatternref))
                (bind _output_get_2 (Variables|Default|SetNextCard _card))
                (Default|CallLocalEventonCard _output_get_2 "(TagName=\"Event.Card.Generate\")" "NewEnumerator2" :!label _label)
                (bind _bhaschanged (CallFunction|HasAppearanceChanged))
                (Variables|Default|SetbAppearanceChanged _bhaschanged)
                (Variables|Default|SetIcon (Default|GetCardPortrait (Variables|Default|GetNextCard) "NewEnumerator2"))
                (Variables|Default|SetTint (.specifiedcolor (Default|GetCardFrameTint (Variables|Default|GetNextCard) "NewEnumerator2")))
                (Variables|Default|SetLastCardRepetitions (Default|GetCardRepetitions (Variables|Default|GetNextCard) "NewEnumerator0"))
                (CallFunction|UpdateTooltipsfromCard (Variables|Default|GetNextCard))
                (if (== (Variables|/Game/ShamanCardGame/Blueprints/Core/BP_Card.BP_Card_C|GetType (Variables|Default|GetNextCard)) "(TagName=\"Effect.Attack\")")
                  (bind _effectvalue (Default|GetCardEffectValue :self (Variables|Default|GetNextCard) :RequiredTags "(GameplayTags=((TagName=\"Effect.Attack\")))"))
                  (Variables|Default|SetStatusValue _effectvalue)
                  (Variables|Default|SetTextAlignment "NewEnumerator3")
                  (else
                    (Variables|Default|SetTextAlignment "NewEnumerator0")))
                (if (Math|Boolean|ORBoolean (== (Variables|Default|GetCurrentEventTag) "(TagName=\"Event.TurnStart\")") (!= (Variables|Default|GetStatusValue) (Variables|Default|GetLastDisplayedStatusValue)) (Variables|Default|GetbAppearanceChanged))
                  (CallFunction|QueueDelay (Variables|Default|GetPreDisplayDelay))
                  (Game|SpawnActorfromClass "/Game/ShamanCardGame/Blueprints/CardActions/BP_Action_ModifyStatus.BP_Action_ModifyStatus_C" (Math|Transform|MakeTransform "0, 0, 0" "0, 0, 0" "1.000000,1.000000,1.000000") "AlwaysSpawn" "OverrideRootScale" 0 self (Variables|Default|GetStatusValue) false false "" true (select (== (Variables|/Game/ShamanCardGame/Blueprints/Core/BP_Card.BP_Card_C|GetType (Variables|Default|GetNextCard)) "(TagName=\"Effect.Attack\")") (select (> (Variables|Default|GetLastCardRepetitions) 0) (Utilities|Text|ToText(String) (Utilities|String|Append (Utilities|String|ToString(Integer) (Variables|Default|GetStatusValue)) "x" (Utilities|String|ToString(Integer) (+ (Variables|Default|GetLastCardRepetitions) 1)))) "") "") true -1.0 0)
                  (Variables|Default|SetLastDisplayedStatusValue (Variables|Default|GetStatusValue))))
              (:else)))
          (:else
            (Development|PrintString "WARNING: No valid card in Attack Pattern Component" true true "(R=1.000000,G=1.000000,B=0.000000,A=1.000000)" 9.0)))))
    (:Event.PostModifyStatus
      (Variables|Default|GetNextCard
        (:then
          (Default|ResetinHandModifications (Variables|Default|GetNextCard))
          (goto _label))
        (:else)))))

(fn HasAppearanceChanged
  (bind _nextcard (Variables|Default|GetNextCard))
  (return (Math|Boolean|ORBoolean (!= (Variables|Default|GetIcon) (Default|GetCardPortrait _nextcard "NewEnumerator2")) (!= (.specifiedcolor (Default|GetCardFrameTint _nextcard "NewEnumerator2")) (Variables|Default|GetTint)) (!= (Default|GetCardRepetitions _nextcard "NewEnumerator0") (Variables|Default|GetLastCardRepetitions)))))

(fn UpdateTooltipsfromCard
  (params (Card :type BP%20Card%20Object%20Reference))
  (for _array_element (Default|GetCardTooltips Card "NewEnumerator0")
    (Utilities|Array|Add (LocalVariables|GetLocalTooltips) (Utilities|Struct|MakeFTooltipValue _array_element false)))
  (Variables|Default|SetTooltips (LocalVariables|GetLocalTooltips))
  (return))