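; A status effect Blueprint in the card game that draws cards for its owner at the start of each turn.
; On BeginPlay it finds the owner's hand pile component and, if one exists, binds to the turn-start event on the owner's dispatcher hub.
; Turn start attempts one draw per point of status value.
; A turn-end branch discards the hand, though only turn start is bound here.
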(event EventBeginPlay
  (bind _returnvalue (Components|GetOwner))
  (bind _returnvalue_2 (Actor|GetComponentbyClass _returnvalue "/Game/ShamanCardGame/Blueprints/Piles/BP_PileComponent_Hand.BP_PileComponent_Hand_C"))
  (|CallParentFunction)
  (if (Utilities|IsValid _returnvalue_2)
    (Variables|Default|SetHandRef _returnvalue_2)
    (Default|BindMultipleEventstoHub (.ReturnValue (CallFunction|GetOwnersDispatcherHub)) self "(GameplayTags=((TagName=\"Event.TurnStart\"),(TagName=\"Event.TurnEnd\")))")))

(event EventRunEvent
  (params (EventTag :type Gameplay%20Tag%20Structure) (CallingObject :type Object%20Object%20Reference%20%28by%20ref%29) (bGlobal :type Boolean) (Payload :type Object%20Object%20Reference%20%28by%20ref%29) (CallTags :type Gameplay%20Tag%20Container%20Structure%20%28by%20ref%29))
  ;[0 0 0] Responsible for drawing new cards to the hand component.
  ; Assumes a hand pile component attached to the same owner (generally the Card Player)
  (|SwitchGameplayTag EventTag
    (:Event.TurnStart
      (for _index (range 0 (- (Variables|Default|GetStatusValue) 1))
        (Default|AttemptDraw (Variables|Default|GetHandRef))))
    (:Event.TurnEnd
      (Default|DiscardHand (Variables|Default|GetHandRef)))))