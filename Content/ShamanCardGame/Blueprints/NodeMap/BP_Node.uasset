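; Clickable node on the card game's node map, showing its map event's icon from a data table.
; Construction builds spline-mesh edges to connected nodes and a dynamic material for icon and color.
; Enabled nodes wobble in a gated timeline loop and highlight white on hover unless the UI blocks the map.
; Clicking records the visit in the game instance, signals selection and runs the event component; CrossOut marks visited nodes.
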(event Custom|CrossOut
  ;[0 0 0] Visualizing node having been visited by crossing it out
  (Rendering|SetVisibility (Variables|Default|GetCrossMesh) true false)
  (Rendering|Material|SetVectorParameterValue (Variables|Default|GetNodeMaterial) "Color" (Variables|Default|GetTrueColor) :!class /Script/Engine.MaterialInstanceDynamic))

(event Custom|Enable
  ;[0 0 0] Signals that node can be clicked and starts wobble animation to communicate this to the player
  (Variables|Default|SetbEnabled true)
  (Utilities|FlowControl|Sequence
    (:then_0
      (goto _label Open))
    (:then_1
      (bind _wobble (Timeline|TL_Wobble PlayFromStart)
        (:Update
          (Transformation|SetRelativeScale3D (Variables|Default|GetNodeMesh) (Math|Conversions|ToVector(Float) (+ 1.0 (* _wobble 0.2)))))
        (:Finished
          (Utilities|FlowControl|Gate true :!label _label
            (:Exit
              (Timeline|TL_Wobble PlayFromStart))))))))

(event Custom|StopEnable
  ;[0 0 0] Signals that node can be clicked and starts wobble animation to communicate this to the player
  (Variables|Default|SetbEnabled false)
  (Utilities|FlowControl|Gate true) ; enters at Close
)

(event EventHoverOverNode
  ;[0 0 0] Handles mouse over highlighting
  (if (Variables|Default|GetbEnabled)
    (if (not (Default|ShouldNodeMapbeBlocked (Variables|/Game/ShamanCardGame/Blueprints/Core/BP_CardPlayer.BP_CardPlayer_C|GetPlayerUI (CallFunction|GetCardPlayerPure))))
      (bind _returnvalue (Rendering|Material|GetVectorParameterValue (Variables|Default|GetNodeMaterial) "Color" :!class /Script/Engine.MaterialInstanceDynamic))
      (Variables|Default|SetTrueColor _returnvalue)
      (Rendering|Material|SetVectorParameterValue (Variables|Default|GetNodeMaterial) "Color" "(R=1.000000,G=1.000000,B=1.000000,A=1.000000)" :!class /Script/Engine.MaterialInstanceDynamic))))

(event EventHoverOffNode
  ;[0 0 0] Handles mouse over highlighting
  (if (Variables|Default|GetbEnabled)
    (Rendering|Material|SetVectorParameterValue (Variables|Default|GetNodeMaterial) "Color" (Variables|Default|GetTrueColor) :!class /Script/Engine.MaterialInstanceDynamic)))

(event EventClickNode
  ;[0 0 0] Resolve result of clicking node
  (if (Variables|Default|GetbEnabled)
    (if (not (Default|ShouldNodeMapbeBlocked (Variables|/Game/ShamanCardGame/Blueprints/Core/BP_CardPlayer.BP_CardPlayer_C|GetPlayerUI (CallFunction|GetCardPlayerPure))))
      (Class|BPICardGameInstance|AddVisitedNodetoInstance(Message) (Game|GetGameInstance) (Variables|Default|GetId))
      (Default|CallOnNodeSelected self)
      (Default|RunMapEvent (Variables|Default|GetMapEventRef) (Variables|Default|GetMapEvent)))))

(event EventBeginPlay
  ;[0 0 0] Store original node color on startup
  (bind _returnvalue (Rendering|Material|GetVectorParameterValue (Variables|Default|GetNodeMaterial) "Color" :!class /Script/Engine.MaterialInstanceDynamic))
  (Variables|Default|SetTrueColor _returnvalue)
  (bind _returnvalue_2 (Game|AddComponentbyClass (Variables|Default|GetMapEventClass)))
  (Variables|Default|SetMapEventRef _returnvalue_2))

(fn ConstructionScript
  (bind _mapevent (Variables|Default|GetMapEvent))
  (bind _nodemesh (Variables|Default|GetNodeMesh))
  (CallFunction|AddConnectionSplines)
  (bind _returnvalue (Rendering|Material|CreateDynamicMaterialInstance _nodemesh 0 (Rendering|Material|GetMaterial _nodemesh 0) "None" :!class /Script/Engine.PrimitiveComponent))
  (Variables|Default|SetNodeMaterial _returnvalue)
  (bind _returnvalue_2 (Utilities|GetDataTableRow (.datatable _mapevent) (.rowname _mapevent))
    (:then
      (Rendering|Material|SetTextureParameterValue (Variables|Default|GetNodeMaterial) "Texture" (.Icon (Utilities|Struct|BreakFMapEvent _returnvalue_2))))))

(fn DisplaySplinePath
  (params (Spline :type Spline%20Component%20Object%20Reference))
  (for _index (range 0 (.ReturnValue (Math|Float|Division(WholeandRemainder) (Spline|GetSplineLength Spline) (LocalVariables|GetDivisor))))
    (bind _returnvalue (AddComponent|AddSplineMeshComponent true))
    (Components|StaticMesh|SetStaticMesh _returnvalue "/Game/ShamanCardGame/Demo/Meshes/SM_Edge.SM_Edge")
    (SplineMesh|SetStartandEnd _returnvalue (Spline|GetLocationatDistanceAlongSpline Spline (* _index (LocalVariables|GetDivisor)) "World") (Spline|GetDirectionatDistanceAlongSpline Spline (* _index (LocalVariables|GetDivisor)) "World") (Spline|GetLocationatDistanceAlongSpline Spline (+ (* _index (LocalVariables|GetDivisor)) (LocalVariables|GetDivisor)) "World") (Spline|GetDirectionatDistanceAlongSpline Spline (+ (* _index (LocalVariables|GetDivisor)) (LocalVariables|GetDivisor)) "World") true :!class /Script/Engine.SplineMeshComponent))
  (return))

(fn AddConnectionSplines
  (bind _returnvalue (Transformation|GetActorLocation))
  (for _array_element (Variables|Default|GetConnections)
    (Utilities|IsValid _array_element
      (:Is%20Valid
        (bind _returnvalue_2 (AddComponent|AddSplineComponent false))
        (Spline|SetLocationatSplinePoint _returnvalue_2 0 (+ _returnvalue (* (Math|Vector|Normalize (- (Transformation|GetActorLocation _array_element) _returnvalue)) 5e+01)) "World" true)
        (Spline|SetLocationatSplinePoint _returnvalue_2 (- (Spline|GetNumberOfSplinePoints _returnvalue_2) 1) (- (Transformation|GetActorLocation _array_element) (* (Math|Vector|Normalize (- (Transformation|GetActorLocation _array_element) _returnvalue)) 5e+01)) "World" true)
        (CallFunction|DisplaySplinePath _returnvalue_2))))
  (return))