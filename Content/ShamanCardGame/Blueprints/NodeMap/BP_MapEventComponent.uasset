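; Base component for node map events that picks random encounters from data tables, with an empty RunMapEvent and a stub GetEncounterTags.
; ChooseRandomEncounter shuffles tables and rows, seeking a row that has all required tags, matches a weighted-random tag and is not a completed story encounter.
; Failed searches drop the picked tag and reroll, then finally retry the last searched rows ignoring completion before reporting failure.
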(event Custom|RunMapEvent
  (params (EventData :type Data%20Table%20Row%20Handle%20Structure)))

(fn ChooseRandomEncounter
  (params (MapEventData :type F%20Map%20Event%20Structure%20%28by%20ref%29))
  (bind (_encountertables _tagweights _requiredtags) (Utilities|Struct|BreakFMapEvent MapEventData))
  (bind _output_get (LocalVariables|SetLocalEncounterTables _encountertables))
  (Utilities|Array|Shuffle _output_get)
  (LocalVariables|SetbLocalNoRequiredTags (== (Utilities|Array|Length (GameplayTags|BreakGameplayTagContainer _requiredtags)) 0))
  (if (> (Utilities|Map|Length _tagweights) 0)
    (LocalVariables|SetLocalTagWeights (Utilities|Struct|BreakFMapEvent MapEventData))
    (bind _cardplayer (CallFunction|GetCardPlayer :!label _label))
    (bind _pickedtags (Default|GetRandomTagsbyWeights (Variables|/Game/ShamanCardGame/Blueprints/Core/BP_CardPlayer.BP_CardPlayer_C|GetBP_ChanceManagerComponent _cardplayer) (LocalVariables|GetLocalTagWeights) 1))
    (LocalVariables|SetLocalPickedTag (Utilities|Array|Get(acopy) _pickedtags))
    (bind _donestoryencounters (Class|BPICardGameInstance|GetDoneStoryEncountersfromInstance(Message) (Game|GetGameInstance) :!label _label_2))
    (LocalVariables|SetLocalDoneStoryEncounters _donestoryencounters)
    (for _array_element (LocalVariables|GetLocalEncounterTables)
      (bind _output_get_2 (LocalVariables|SetLocalEncounterTable _array_element))
      (bind _outrownames (DataTable|GetDataTableRowNames _output_get_2))
      (bind _output_get_3 (LocalVariables|SetLocalEncounterRows _outrownames))
      (Utilities|Array|Shuffle _output_get_3)
      (for _array_element_2 (LocalVariables|GetLocalEncounterRows)
        (bind _tags (CallFunction|GetEncounterTags (LocalVariables|GetLocalEncounterTable) _array_element_2))
        (if (and (or (LocalVariables|GetbLocalNoTagWeights) (GameplayTags|HasTag _tags (LocalVariables|GetLocalPickedTag) true)) (or (LocalVariables|GetbLocalNoRequiredTags) (GameplayTags|HasAllTags _tags (Utilities|Struct|BreakFMapEvent MapEventData) true)))
          (if (not (Utilities|Array|ContainsItem (LocalVariables|GetLocalDoneStoryEncounters) (Utilities|Struct|MakeDataTableRowHandle (LocalVariables|GetLocalEncounterTable) _array_element_2)))
            (return true (Utilities|Struct|MakeDataTableRowHandle (LocalVariables|GetLocalEncounterTable) _array_element_2))))))
    (if (> (Utilities|Map|Length (LocalVariables|GetLocalTagWeights)) 1)
      (Utilities|Map|Remove (LocalVariables|GetLocalTagWeights) (LocalVariables|GetLocalPickedTag))
      (goto _label)
      (else
        _))
    (else
      (LocalVariables|SetbLocalNoTagWeights true)
      (goto _label_2)))
  (if (LocalVariables|GetbLocalRetryAndIgnoreDone)
    (return false "")
    (else
      (LocalVariables|SetbLocalRetryAndIgnoreDone true)
      (Utilities|Array|Clear (LocalVariables|GetLocalDoneStoryEncounters))
      (for _array_element_3 (LocalVariables|GetLocalEncounterRows)
        (bind _tags_2 (CallFunction|GetEncounterTags (LocalVariables|GetLocalEncounterTable) _array_element_3))
        (if (and (or (LocalVariables|GetbLocalNoTagWeights) (GameplayTags|HasTag _tags_2 (LocalVariables|GetLocalPickedTag) true)) (or (LocalVariables|GetbLocalNoRequiredTags) (GameplayTags|HasAllTags _tags_2 (Utilities|Struct|BreakFMapEvent MapEventData) true)))
          (if (not (Utilities|Array|ContainsItem (LocalVariables|GetLocalDoneStoryEncounters) (Utilities|Struct|MakeDataTableRowHandle (LocalVariables|GetLocalEncounterTable) _array_element_3)))
            (return true (Utilities|Struct|MakeDataTableRowHandle (LocalVariables|GetLocalEncounterTable) _array_element_3))))))))

(fn GetEncounterTags
  (params (DataTable :type Data%20Table%20Object%20Reference) (RowName :type Name))
  (return ""))