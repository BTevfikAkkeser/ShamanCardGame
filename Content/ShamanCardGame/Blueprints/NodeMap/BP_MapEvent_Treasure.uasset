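; Treasure node event for the card game's node map, which grants a reward by playing a card.
; RunMapEvent spawns a BP_Card from RewardCardData, attempts to use it immediately, saves the game with the deck and listens on the global dispatcher hub for Event.CloseRewardScreen.
; RunEvent saves again and unbinds that listener.
; GetEncounterTags reads gameplay tags from a data table row, while friendly name and priority return empty defaults.
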(event EventRunEvent
  (params (EventTag :type Gameplay%20Tag%20Structure) (CallingObject :type Object%20Object%20Reference%20%28by%20ref%29) (bGlobal :type Boolean) (Payload :type Object%20Object%20Reference%20%28by%20ref%29) (CallTags :type Gameplay%20Tag%20Container%20Structure%20%28by%20ref%29))
  (|SwitchGameplayTag EventTag
    (:Event.CloseRewardScreen
      (Class|BPICardGameInstance|AttemptSaveGame(Message) (Game|GetGameInstance) "" true)
      (CallFunction|UnbindEventfromGlobalDispatcherHub self "(TagName=\"Event.CloseRewardScreen\")"))))

(event EventRunMapEvent
  (params (EventData :type Data%20Table%20Row%20Handle%20Structure))
  (bind _returnvalue (Game|SpawnActorfromClass "/Game/ShamanCardGame/Blueprints/Core/BP_Card.BP_Card_C" (Math|Transform|MakeTransform "0, 0, 0" "0, 0, 0" "1.000000,1.000000,1.000000") "AlwaysSpawn" "OverrideRootScale" 0 (CallFunction|MakeCardStructfromCardData (Variables|Default|GetRewardCardData)) 0))
  (Default|AttemptUseCard _returnvalue (Utilities|Array|MakeArray 0) false false false)
  (Class|BPICardGameInstance|AttemptSaveGame(Message) (Game|GetGameInstance) "" true)
  (CallFunction|BindEventtoGlobalDispatcherHub self "(TagName=\"Event.CloseRewardScreen\")"))

(fn GetEncounterTags
  (params (DataTable :type Data%20Table%20Object%20Reference) (RowName :type Name :default "None"))
  (bind _returnvalue (Utilities|GetDataTableRow DataTable RowName)
    (:then
      (return (.GameplayTags (Utilities|Struct|BreakFStoryEncounter _returnvalue))))))

(fn GetFriendlyName
  (return ""))

(fn GetPriority
  (return 0.0))