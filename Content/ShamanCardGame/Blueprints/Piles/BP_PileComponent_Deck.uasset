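; Deck pile component that builds the deck of cards at BeginPlay in the card game.
; After a one-tick delay, it spawns cards from the game instance's saved deck, falling back to a DeckData table row.
; It hands the cards to the owner's draw pile component and sets each card's owner to the minion with the matching unique ID.
; It then broadcasts DeckSetupDone through the global dispatcher hub, twice on the game-instance path.
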(event Custom|SetupCardsInDrawPile
  (Default|AssignExistingCards (Actor|GetComponentbyClass (Components|GetOwner) "/Game/ShamanCardGame/Blueprints/Piles/BP_PileComponent_Draw.BP_PileComponent_Draw_C") (Variables|Default|GetCards))
  (for _array_element (Variables|Default|GetCards)
    (bind _outactors (Actor|GetAllActorsOfClass "/Game/ShamanCardGame/Blueprints/Core/BP_Minion.BP_Minion_C"))
    (for _array_element_2 _outactors
      (if (Utilities|Enum|Equal(Enum) (Utilities|Struct|BreakFMinion (Variables|/Game/ShamanCardGame/Blueprints/Core/BP_Minion.BP_Minion_C|GetMinionData _array_element_2)) (Default|GetCardOwnerID _array_element "NewEnumerator1"))
        (Actor|SetOwner _array_element _array_element_2))))
  (CallFunction|CallEventinGlobalDispatcherHub "(TagName=\"Event.DeckSetupDone\")" self))

(event EventBeginPlay
  (bind _deckdata (Variables|Default|GetDeckData))
  (Utilities|FlowControl|Delay 0.0)
  (bind (_bsuccess _deck) (Class|BPICardGameInstance|GetDeckfromInstance(Message) (Game|GetGameInstance)))
  (if _bsuccess
    (for _array_element _deck
      (bind _returnvalue (Game|SpawnActorfromClass "/Game/ShamanCardGame/Blueprints/Core/BP_Card.BP_Card_C" (Transformation|GetActorTransform (Components|GetOwner)) "AlwaysSpawn" "OverrideRootScale" 0 _array_element 0))
      (CallFunction|AttemptAddExistingCard _returnvalue))
    (CallFunction|SetupCardsinDrawPile)
    (CallFunction|CallEventinGlobalDispatcherHub "(TagName=\"Event.DeckSetupDone\")" self)
    (else
      (bind _returnvalue_2 (Utilities|GetDataTableRow (.datatable _deckdata) (.rowname _deckdata))
        (:then
          (for _array_element_2 (Utilities|Struct|BreakFDeck _returnvalue_2)
            (CallFunction|SpawnandAddNewCard _array_element_2))
          (CallFunction|SetupCardsinDrawPile))))))