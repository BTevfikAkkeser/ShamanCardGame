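; Pile component for the player's hand in a card game, handling draws, end of turn and cards entering or leaving the hand.
; Draws fire a Draw event on a specified, random or first card from a source pile, reshuffling discard into an empty draw pile.
; Enter/exit events and a global ModifyInHand listener drive card behavior and modifier resets.
; It also exhausts cards owned by a given actor.
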(event Custom|AttemptDraw
  (if (> (Variables|Default|GetMaxPileSize) (Utilities|Array|Length (Variables|Default|GetCards)))
    (CallFunction|DrawCard 0 "/Game/ShamanCardGame/Blueprints/Piles/BP_PileComponent_Draw.BP_PileComponent_Draw_C")))

(event EventBeginPlay
  (CallFunction|BindMultipleEventstoGlobalDispatcherHub self "(GameplayTags=((TagName=\"Event.Card.ModifyInHand\")))"))

(event EventRunEvent
  (params (EventTag :type Gameplay%20Tag%20Structure) (CallingObject :type Object%20Object%20Reference%20%28by%20ref%29) (bGlobal :type Boolean) (Payload :type Object%20Object%20Reference%20%28by%20ref%29) (CallTags :type Gameplay%20Tag%20Container%20Structure%20%28by%20ref%29))
  (|SwitchGameplayTag EventTag
    (:Event.Card.ModifyInHand
      (bind _asbp_card (Utilities|Casting|CastToBP_Card CallingObject))
      (Default|ResetinHandModifications _asbp_card))))

(fn AttemptAddExistingCard
  (params (Card :type BP%20Card%20Object%20Reference%20%28by%20ref%29))
  (bind _bsuccess (|CallParentFunction Card))
  (if _bsuccess
    (Default|CallLocalEventonCard Card "(TagName=\"Event.Card.EnterHand\")" "NewEnumerator2")
    (return true)
    (else
      (return false))))

(fn GetPriority
  (return 1e+02))

(fn DrawCard
  (params (SpecifiedCard :type BP%20Card%20Object%20Reference) (SourcePile :type BP%20Pile%20Component%20Class%20Reference))
  (bind _returnvalue (Components|GetOwner))
  (bind _returnvalue_2 (Actor|GetComponentbyClass _returnvalue SourcePile))
  (bind _cards (Variables|/Game/ShamanCardGame/Blueprints/Piles/BP_PileComponent.BP_PileComponent_C|GetCards _returnvalue_2))
  (if (> (Utilities|Array|Length (Variables|/Game/ShamanCardGame/Blueprints/Piles/BP_PileComponent.BP_PileComponent_C|GetCards (Actor|GetComponentbyClass (Components|GetOwner) SourcePile))) 0)
    _
    (elif (== SourcePile "/Game/ShamanCardGame/Blueprints/Piles/BP_PileComponent_Draw.BP_PileComponent_Draw_C")
      (Default|ReshuffleDiscardIntoDraw (Actor|GetComponentbyClass (Components|GetOwner) "/Game/ShamanCardGame/Blueprints/Piles/BP_PileComponent_Draw.BP_PileComponent_Draw_C"))
      (if (> (Utilities|Array|Length (Variables|/Game/ShamanCardGame/Blueprints/Piles/BP_PileComponent.BP_PileComponent_C|GetCards (Actor|GetComponentbyClass (Components|GetOwner) SourcePile))) 0)
        _
        (else
          (return false 0)))
      (else
        (return false 0))))
  (LocalVariables|GetSpecifiedCard
    (:then
      (if (> (Utilities|Array|FindItem _cards SpecifiedCard) -1)
        (Variables|Default|SetDrawnCard SpecifiedCard)
        (else
          (Variables|Default|SetDrawnCard (select (Variables|Default|GetbRandomDrawOrder) (.OutItem (Utilities|Array|Random _cards)) (Utilities|Array|Get(acopy) _cards)) :!label _label))))
    (:else
      (goto _label)))
  (bind _bsuccess (Default|CallEvent (Variables|/Game/ShamanCardGame/Blueprints/Core/BP_Card.BP_Card_C|GetBP_DispatcherHubComponent_Local (Variables|Default|GetDrawnCard)) "(TagName=\"Event.Card.Draw\")" (Variables|Default|GetDrawnCard) 0 "NewEnumerator1"))
  (return _bsuccess (Variables|Default|GetDrawnCard)))

(fn RemoveAllCardsOwnedbyActor
  (params (Actor :type Actor%20Object%20Reference))
  (bind _cardplayer (CallFunction|GetCardPlayer))
  (bind _arrayelement (Utilities|Array|ReverseforEachLoop (Variables|Default|GetCards))
    (:LoopBody
      (if (== (Components|GetOwner _arrayelement) Actor)
        (bind _output_get (LocalVariables|SetLocalCard _arrayelement))
        (CallFunction|TransferCardtoPile _output_get (Variables|/Game/ShamanCardGame/Blueprints/Core/BP_CardPlayer.BP_CardPlayer_C|GetBP_PileComponent_Exhaust _cardplayer))
        (CallFunction|QueueEventinGlobalDispatcherHub "(TagName=\"Event.Action.Exhaust\")" (LocalVariables|GetLocalCard) 0 -1.0)))
    (:Completed
      (return))))

(fn DiscardHand
  (bind _output_get (LocalVariables|SetLocalCards (Variables|Default|GetCards)))
  (for _array_element _output_get
    (Default|RunEndTurnEvent _array_element "(GameplayTags=((TagName=\"Flag.Passive\")))"))
  (return))

(fn RequestRemoveCardfromPile
  (params (Card :type BP%20Card%20Object%20Reference%20%28by%20ref%29))
  (|CallParentFunction Card)
  (Default|CallLocalEventonCard Card "(TagName=\"Event.Card.ExitHand\")" "NewEnumerator2")
  (Default|ResetinHandModifications Card)
  (return true))