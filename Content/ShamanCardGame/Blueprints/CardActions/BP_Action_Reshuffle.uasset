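; Card action that visualizes a reshuffle, flying card widgets from the discard pile to the draw pile.
; PlayAction spawns one hand-created widget per card on a delayed loop, lowering the displayed discard count as each departs.
; Each widget follows a Bezier path through a reshuffle anchor with speed and scale curves.
; Its removal callback raises the displayed draw count, and the last card's removal ends the action.
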(event Custom|UpdateDrawOnReach
  (params (RemovedCard :type BP%20Card%20Object%20Reference) (RemovedWidget :type Widget%20Object%20Reference))
  (bind _cards (Variables|Default|GetCards))
  ;[0 0 0] Tells card hand to create card widgets and animate them moving from the discard to the draw pile, updaing the card amounts displayed when they should visually occur
  (Default|UpdatePileWidgetAmount (Variables|Default|GetPlayerUiRef) "(TagName=\"Pile.Draw\")" (+ (Utilities|Array|FindItem (Variables|Default|GetCards) RemovedCard) 1))
  (if (== RemovedCard (Utilities|Array|Get(acopy) _cards (Utilities|Array|LastIndex _cards)))
    (CallFunction|EndAction)))

(event EventSetupAction
  ;[0 0 0] Tells card hand to create card widgets and animate them moving from the discard to the draw pile, updaing the card amounts displayed when they should visually occur
  (bind _cardplayer (CallFunction|GetCardPlayer))
  (bind _output_get (Variables|Default|SetCardPlayerRef _cardplayer))
  (bind _output_get_2 (Variables|Default|SetPlayerUiRef (Variables|/Game/ShamanCardGame/Blueprints/Core/BP_CardPlayer.BP_CardPlayer_C|GetPlayerUI _output_get)))
  (Variables|Default|SetHandWidgetRef (Variables|/Game/ShamanCardGame/Widgets/WBP_Layout_RLDB.WBP_Layout_RLDB_C|GetWBP_Hand _output_get_2)))

(event EventPlayAction
  (bind _playeruiref (Variables|Default|GetPlayerUiRef))
  ;[0 0 0] Tells card hand to create card widgets and animate them moving from the discard to the draw pile, updaing the card amounts displayed when they should visually occur
  (bind _viewportposition (Default|GetAnchorWidgetPosition (Variables|Default|GetHandWidgetRef) "(TagName=\"Pile.Discard\")"))
  (Variables|Default|SetDiscardPilePosition _viewportposition)
  (bind _viewportposition_2 (Default|GetAnchorWidgetPosition (Variables|Default|GetHandWidgetRef) "(TagName=\"Pile.Draw\")"))
  (Variables|Default|SetDrawPilePosition _viewportposition_2)
  (bind (_arrayelement _arrayindex) (Utilities|ForEachLoopDelayed (Variables|Default|GetCards) 1 (Variables|Default|GetCardDelay))
    (:LoopBody
      (Default|UpdatePileWidgetAmount (Variables|Default|GetPlayerUiRef) "(TagName=\"Pile.Discard\")" (- (Utilities|Array|LastIndex (Variables|Default|GetCards)) _arrayindex))
      (bind _createdcardwidget (Default|CreateandSetupCardWidget (Variables|Default|GetHandWidgetRef) _arrayelement (Utilities|Struct|MakeWidgetTransform (Variables|Default|GetDiscardPilePosition) "(X=0.000000,Y=0.000000)" "(X=0.000000,Y=0.000000)" 0.0) false))
      (Utilities|Array|Add (Variables|Default|GetCardWidgets) _createdcardwidget)
      (EventDispatchers|BindEventtoOnRemoved _createdcardwidget (delegate Custom|UpdateDrawOnReach))
      (Default|SetupBezierFollow _createdcardwidget (Utilities|Struct|MakeFTransferAnim (Variables|/Game/ShamanCardGame/Widgets/WBP_Layout_RLDB.WBP_Layout_RLDB_C|GetWBP_CardListButton_Discard _playeruiref) (Variables|/Game/ShamanCardGame/Widgets/WBP_CardHand.WBP_CardHand_C|GetWBP_ReshuffleAnchor (Variables|/Game/ShamanCardGame/Widgets/WBP_Layout_RLDB.WBP_Layout_RLDB_C|GetWBP_Hand _playeruiref)) (Variables|/Game/ShamanCardGame/Widgets/WBP_Layout_RLDB.WBP_Layout_RLDB_C|GetWBP_CardListButton_Draw _playeruiref) 0.8 "/Game/ShamanCardGame/Blueprints/Curves/Curve_Decelerate_Float.Curve_Decelerate_Float" "/Game/ShamanCardGame/Blueprints/Curves/Curve_Parabel_Float.Curve_Parabel_Float" 0.5 -0.5 "(X=40.000000,Y=40.000000)")))))

(fn ConstructionScript
  (|CallParentFunction))