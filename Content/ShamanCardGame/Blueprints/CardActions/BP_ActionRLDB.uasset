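; BP_ActionRLDB is the base actor for card game actions that visualize gameplay to the player, with behavior supplied by child blueprints.
; On BeginPlay it runs SetupAction to cache data early, then queues itself with BP_ActionManagerRLDB.
; The manager calls AnimateAction, which runs PlayAction; overrides must finish with EndAction, which applies an optional delay and tells the manager to proceed, otherwise the game hangs.
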(event Custom|PlayAction
  (CallFunction|EndAction) ; End Action should always be called at the end of PlayAction, or the action manager, causing the game to hang
)

(event Custom|SetupAction
  ;[0 0 0 1 12] For overriding in child blueprints. For running any setup code immediately when the action is spawned.
  ; Useful if you want to access variables from actors that can be destroyed between when an action is
  ; queued and when it is run. If so you can access them here and store them in variables to be used when
  ; playing the action
)

(event EventAnimateAction
  (params (CallingActionManager :type Object%20Object%20Reference))
  (Variables|Default|SetActionManagerRef CallingActionManager)
  (CallFunction|PlayAction))

(event EventEndAction
  (if (>= (Variables|Default|GetEndDelay) 0.0)
    (Utilities|FlowControl|Delay (Variables|Default|GetEndDelay)))
  (Class|BPICardActionManager|ProceedfromOngoingAction(Message) (Variables|Default|GetActionManagerRef) self))

(event EventBeginPlay
  (CallFunction|SetupAction)
  (bind _returnvalue (Actor|GetActorOfClass "/Game/ShamanCardGame/Blueprints/Core/BP_ActionManagerRLDB.BP_ActionManagerRLDB_C"))
  (Default|QueueAction _returnvalue self))

(fn ConstructionScript)

(fn AttemptDestroyAction
  (Actor|DestroyActor)
  (return true))