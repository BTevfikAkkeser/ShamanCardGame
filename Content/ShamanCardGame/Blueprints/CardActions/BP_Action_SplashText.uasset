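; BP_Action_SplashText is a card action in the shaman card game that shows splash text over a target puppet.
; On play, it spawns a BP_TextSplash actor slightly above the puppet's relative center-message point, offset from the puppet's location.
; It passes its display text and sRGB-converted color to the splash, then ends the action immediately after spawning.
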(event EventPlayAction
  (bind _puppet (Variables|Default|GetPuppet))
  ;[0 0 0] Displays the input splash text at the center of the input puppet
  (bind _relativecenter (Class|BPICardPuppet|GetPuppetRelativeCenter(Message) _puppet))
  (Game|SpawnActorfromClass "/Game/ShamanCardGame/Blueprints/UI/BP_TextSplash.BP_TextSplash_C" (Math|Transform|MakeTransform (+ (+ _relativecenter (Transformation|GetActorLocation _puppet)) "0, 0,70.000000") "0, 0, 0" "1.000000,1.000000,1.000000") "Undefined" "OverrideRootScale" 0 (Variables|Default|GetDisplayText) (Math|Conversions|ToColor(LinearColor) (Variables|Default|GetColor)) 0)
  (CallFunction|EndAction))

(fn ConstructionScript
  (|CallParentFunction))