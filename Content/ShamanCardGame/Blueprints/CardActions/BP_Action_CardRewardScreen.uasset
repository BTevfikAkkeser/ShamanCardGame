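; Card action that shows the player's card reward screen with a set of card options, a title and an optional skip.
; PlayAction binds to the screen's return-selected-card event on the player UI, then updates the screen from the action's variables.
; The action ends when that event fires, without using the selected card or skip result itself.
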(event Custom|ContinueActionOnCardSelect
  (params (bSkipped :type Boolean) (Card :type BP%20Card%20Object%20Reference))
  ;[0 0 0] Shows a reward screen that displays card reward options
  (CallFunction|EndAction))

(event EventPlayAction
  ;[0 0 0] Shows a reward screen that displays card reward options
  (bind _cardplayer (CallFunction|GetCardPlayer))
  (EventDispatchers|BindEventtoOnReturnSelectedCard (Variables|/Game/ShamanCardGame/Widgets/WBP_Layout_RLDB.WBP_Layout_RLDB_C|GetWBP_CardRewardScreen (Variables|/Game/ShamanCardGame/Blueprints/Core/BP_CardPlayer.BP_CardPlayer_C|GetPlayerUI _cardplayer)) (delegate Custom|ContinueActionOnCardSelect))
  (Default|UpdateRewardScreen (Variables|/Game/ShamanCardGame/Widgets/WBP_Layout_RLDB.WBP_Layout_RLDB_C|GetWBP_CardRewardScreen (Variables|/Game/ShamanCardGame/Blueprints/Core/BP_CardPlayer.BP_CardPlayer_C|GetPlayerUI _cardplayer)) (Variables|Default|GetCardOptions) (Variables|Default|GetScreenText) (Variables|Default|GetbAllowSkip)))

(fn ConstructionScript
  (|CallParentFunction))