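; Card-game action that fires a Dispatcher Hub event from within the action queue, meant for purely visual events such as showing a card being drawn.
; On play, it passes its event tag, calling object, target flags, payload and call tags to the hub's ResolveCallEvent, then ends immediately.
; Gameplay logic, like adding the card to the hand's array, is intended to stay outside such actions.
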(event EventPlayAction
  ;[0 0 0] For calling events in a Dispatcher Hub that are set up to be called as part of the action queue.
  ;
  ; Generally for calling events that are purely visual, such as showing a card being drawn (as opposed to the gameplay logic of a card being added to the Cards array of the Hand Pile, which should not be handled within actions)
  (Default|ResolveCallEvent (Variables|Default|GetDispatcherHub) (Variables|Default|GetEvent) (Variables|Default|GetCallingObject) (Variables|Default|GetCallSpecificObject) (Variables|Default|GetAlsoCallGlobal) (Variables|Default|GetPayload) (Variables|Default|GetCall%20Tags))
  (CallFunction|EndAction))

(fn ConstructionScript
  (|CallParentFunction))