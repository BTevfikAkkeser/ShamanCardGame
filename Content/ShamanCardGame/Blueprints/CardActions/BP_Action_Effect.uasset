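; Card action that plays the visuals when a card effect triggers, serving as an overridable base for effect types.
; It animates the source puppet and waits for its animation event, or uses an optional start delay when no animation or puppet is available.
; It then spawns the effect's particles at the target's center, nudged horizontally toward the camera, and ends the action without waiting for them.
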(event Custom|SpawnEffectParticles
  ;[0 0 0] Spawn Vfx
  (Variables|Default|GetTarget
    (:then
      (if (Utilities|IsValid (CallFunction|GetEffectParticle (Variables|Default|GetEffect)))
        (bind _relativecenter (Class|BPICardPuppet|GetPuppetRelativeCenter(Message) (Variables|Default|GetTarget)))
        (Niagara|SpawnSystematLocation (CallFunction|GetEffectParticle (Variables|Default|GetEffect)) (Math|Vector|MakeVector (.x (Math|Vector|Lerp(Vector) (+ _relativecenter (Transformation|GetActorLocation (Variables|Default|GetTarget))) (Camera|GetCameraLocation (Game|GetPlayerCameraManager 0)) 0.2)) (.y (Math|Vector|Lerp(Vector) (+ _relativecenter (Transformation|GetActorLocation (Variables|Default|GetTarget))) (Camera|GetCameraLocation (Game|GetPlayerCameraManager 0)) 0.2)) (.Z (Math|Vector|BreakVector (+ _relativecenter (Transformation|GetActorLocation (Variables|Default|GetTarget)))))))
        (CallFunction|EndAction)
        (else
          (CallFunction|EndAction))))
    (:else
      (CallFunction|EndAction))))

(event Custom|CheckAnimationEvent
  (params (Puppet :type Actor%20Object%20Reference) (Animation :type Gameplay%20Tag%20Structure))
  ;[0 0 0] Animate the Puppet
  (if (== Animation (Variables|Default|GetHeroAnim))
    (EventDispatchers|UnbindEventfromOnAnimationEvent (Actor|GetComponentbyClass (stale EventPlayAction _sourcepuppet) "/Game/ShamanCardGame/Blueprints/Core/BP_PuppetComponent.BP_PuppetComponent_C") (delegate Custom|CheckAnimationEvent))
    (CallFunction|SpawnEffectParticles)))

(event EventPlayAction
  ;[0 0 0] Animate the Puppet
  (if (GameplayTags|IsGameplayTagValid (Variables|Default|GetHeroAnim))
    (bind _sourcepuppet (Variables|Default|GetSourcePuppet)
      (:then
        (EventDispatchers|BindEventtoOnAnimationEvent (Actor|GetComponentbyClass _sourcepuppet "/Game/ShamanCardGame/Blueprints/Core/BP_PuppetComponent.BP_PuppetComponent_C") (delegate Custom|CheckAnimationEvent))
        (Class|BPICardPuppet|AnimatePuppet(Message) (Variables|Default|GetSourcePuppet) (Variables|Default|GetHeroAnim)))
      (:else
        (if (>= (Variables|Default|GetStartDelayIfNoAnim) 0.0) :!label _label
          (Utilities|FlowControl|Delay (Variables|Default|GetStartDelayIfNoAnim))
          (CallFunction|SpawnEffectParticles)
          (else
            (CallFunction|SpawnEffectParticles)))))
    (else
      (goto _label))))

(fn ConstructionScript
  (|CallParentFunction))