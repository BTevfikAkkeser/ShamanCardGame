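; Card action that visually transfers a card between two piles in the card game.
; On setup it snapshots the card counts of the source and target piles from the card player.
; On play it has the Hand widget run the transfer animation, updates both pile widgets with those counts, then ends immediately without waiting for the animation.
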(event EventSetupAction
  ;[0 0 0] Handles visually transferring a card from one pile to another. Tells the Hand widget to play transfer animations and updates the amounts displayed in pile widgets
  (bind _cardplayer (CallFunction|GetCardPlayer))
  (if (.bSuccess (Default|GetPilewithPileTag _cardplayer (Variables|Default|GetSourcePile)))
    (Variables|Default|SetSourcePileAmount (Utilities|Array|Length (Variables|/Game/ShamanCardGame/Blueprints/Piles/BP_PileComponent.BP_PileComponent_C|GetCards (.Pile (Default|GetPilewithPileTag _cardplayer (Variables|Default|GetSourcePile)))))))
  (if (.bSuccess (Default|GetPilewithPileTag _cardplayer (Variables|Default|GetTargetPile)))
    (Variables|Default|SetTargetPileAmount (Utilities|Array|Length (Variables|/Game/ShamanCardGame/Blueprints/Piles/BP_PileComponent.BP_PileComponent_C|GetCards (.Pile (Default|GetPilewithPileTag _cardplayer (Variables|Default|GetTargetPile))))))))

(event EventPlayAction
  ;[0 0 0] Handles visually transferring a card from one pile to another. Tells the Hand widget to play transfer animations and updates the amounts displayed in pile widgets
  (bind _cardplayer (CallFunction|GetCardPlayer))
  (Default|TransferCardAction (Variables|/Game/ShamanCardGame/Widgets/WBP_Layout_RLDB.WBP_Layout_RLDB_C|GetWBP_Hand (Variables|/Game/ShamanCardGame/Blueprints/Core/BP_CardPlayer.BP_CardPlayer_C|GetPlayerUI _cardplayer)) (Variables|Default|GetCard) (Variables|Default|GetSourcePile) (Variables|Default|GetTargetPile))
  (Default|UpdatePileWidgetAmount (Variables|/Game/ShamanCardGame/Blueprints/Core/BP_CardPlayer.BP_CardPlayer_C|GetPlayerUI _cardplayer) (Variables|Default|GetSourcePile) (Variables|Default|GetSourcePileAmount))
  (Default|UpdatePileWidgetAmount (Variables|/Game/ShamanCardGame/Blueprints/Core/BP_CardPlayer.BP_CardPlayer_C|GetPlayerUI _cardplayer) (Variables|Default|GetTargetPile) (Variables|Default|GetTargetPileAmount))
  (CallFunction|EndAction))

(fn ConstructionScript
  (|CallParentFunction))