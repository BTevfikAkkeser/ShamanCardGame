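; Blueprint function library of getters for the CardEffect struct in the shaman card game.
; Each function takes a CardEffect and returns a single field, covering effect class and value, target component, gameplay tags, targeting, particle, hero animation and used data.
; It holds no other logic, only direct field reads.
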(fn GetEffectClass
  (params (CardEffect :type F%20Card%20Effect%20Structure))
  (return (.EffectClass (Utilities|Struct|BreakFCardEffect CardEffect))))

(fn GetEffectValue
  (params (CardEffect :type F%20Card%20Effect%20Structure))
  (return (.EffectValue (Utilities|Struct|BreakFCardEffect CardEffect))))

(fn GetEffectTargetComponent
  (params (CardEffect :type F%20Card%20Effect%20Structure))
  (return (.TargetComponent (Utilities|Struct|BreakFCardEffect CardEffect))))

(fn GetEffectGameplayTags
  (params (CardEffect :type F%20Card%20Effect%20Structure))
  (return (.GameplayTags (Utilities|Struct|BreakFCardEffect CardEffect))))

(fn GetEffectTargeting
  (params (CardEffect :type F%20Card%20Effect%20Structure))
  (return (.Targeting (Utilities|Struct|BreakFCardEffect CardEffect))))

(fn GetEffectParticle
  (params (CardEffect :type F%20Card%20Effect%20Structure))
  (return (.Particle (Utilities|Struct|BreakFCardEffect CardEffect))))

(fn GetEffectHeroAnim
  (params (CardEffect :type F%20Card%20Effect%20Structure))
  (return (.HeroAnim (Utilities|Struct|BreakFCardEffect CardEffect))))

(fn GetEffectUsedData
  (params (CardEffect :type F%20Card%20Effect%20Structure))
  (return (.UsedData (Utilities|Struct|BreakFCardEffect CardEffect))))