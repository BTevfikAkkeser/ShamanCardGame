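; Blueprint function library of general helpers for the card game: max integer, Vector2D lerp, set/add/subtract on integers, gameplay tag queries and camera-facing actor rotation.
; Bezier helpers evaluate a quadratic curve with nested lerps, from either 2D points or three widgets, returning position and a tangent angle sampled at a slightly higher alpha.
; Widget positions come from converting render translation through tick-space geometry into viewport coordinates.
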(fn GetHighestPossibleInteger
  (return 2147483647))

(fn LerpVector2D
  (params (A :type Vector%202D%20Structure) (B :type Vector%202D%20Structure) (Alpha :type Float%20%28double-precision%29))
  (return (Math|Vector2D|MakeVector2D (Math|Float|Lerp (.x A) (.x B) Alpha) (Math|Float|Lerp (.y A) (.y B) Alpha))))

(fn GetPlayerCameraLocation
  (return (Camera|GetCameraLocation (Game|GetPlayerCameraManager 0))))

(fn FaceCamera
  (params (Actor :type Actor%20Object%20Reference))
  (Transformation|SetActorRotation Actor (Math|Rotator|FindLookatRotation (Transformation|GetActorLocation Actor) (Camera|GetCameraLocation (Game|GetPlayerCameraManager 0))))
  (return))

(fn GetManipulatedIntValue
  (params (Target :type Integer) (Modifier :type Integer) (Manipulation :type EManipulation%20Enum :default "NewEnumerator2"))
  (return (Utilities|Select :Index Manipulation :NewEnumerator2 Modifier :NewEnumerator0 (+ Target Modifier) :NewEnumerator1 (- Target Modifier))))

(fn GetFirstTagMatchingParentTag
  (params (GameplayTags :type Gameplay%20Tag%20Container%20Structure) (ParentTag :type Gameplay%20Tag%20Structure))
  (switch int (GameplayTags|GetNumGameplayTagsinContainer GameplayTags)
    (:Default
      (for _array_element (.gameplaytags GameplayTags)
        (if (GameplayTags|MatchesTag _array_element ParentTag)
          (return true _array_element)))
      (return false ""))
    (:0
      (return false ""))
    (:1
      (if (GameplayTags|HasTag GameplayTags ParentTag)
        (return true (Utilities|Array|Get(acopy) (.gameplaytags GameplayTags)))))))

(fn IsGameplayTagContainerEmpty
  (params (GameplayTagContainer :type Gameplay%20Tag%20Container%20Structure))
  (return (== (Utilities|Array|Length (.gameplaytags GameplayTagContainer)) 0)))

(fn GetPositionandAngleatBezierAlpha
  (params (Alpha :type Float%20%28double-precision%29) (StartPoint :type Vector%202D%20Structure) (MidPoint :type Vector%202D%20Structure) (EndPoint :type Vector%202D%20Structure))
  (bind _returnvalue (CallFunction|LerpVector2D StartPoint MidPoint Alpha))
  (bind _returnvalue_2 (CallFunction|LerpVector2D MidPoint EndPoint Alpha))
  (bind _returnvalue_3 (+ Alpha 0.001))
  (bind _returnvalue_4 (CallFunction|LerpVector2D StartPoint MidPoint _returnvalue_3))
  (bind _returnvalue_5 (CallFunction|LerpVector2D MidPoint EndPoint _returnvalue_3))
  (bind _returnvalue_6 (CallFunction|LerpVector2D _returnvalue _returnvalue_2 Alpha))
  (bind (_x _y) (Math|Vector2D|BreakVector2D _returnvalue_6))
  (bind _returnvalue_7 (CallFunction|LerpVector2D _returnvalue_4 _returnvalue_5 _returnvalue_3))
  (return _returnvalue_6 (.yaw (Math|Rotator|FindLookatRotation (Math|Vector|MakeVector _x _y 0.0) (Math|Vector|MakeVector (.x _returnvalue_7) (.y _returnvalue_7) 0.0)))))

(fn GetPositionandAngleatBezierAlphaBetweenWidgets
  (params (Alpha :type Float%20%28double-precision%29) (StartWidget :type Widget%20Object%20Reference) (MidWidget :type Widget%20Object%20Reference) (EndWidget :type Widget%20Object%20Reference))
  (bind _viewportposition (CallFunction|GetWidgetTickSpacePosition EndWidget))
  (bind _viewportposition_2 (CallFunction|GetWidgetTickSpacePosition StartWidget))
  (bind _viewportposition_3 (CallFunction|GetWidgetTickSpacePosition MidWidget))
  (bind _returnvalue (CallFunction|LerpVector2D _viewportposition_2 _viewportposition_3 Alpha))
  (bind _returnvalue_2 (CallFunction|LerpVector2D _viewportposition_3 _viewportposition Alpha))
  (bind _returnvalue_3 (+ Alpha 0.001))
  (bind _returnvalue_4 (CallFunction|LerpVector2D _viewportposition_2 _viewportposition_3 _returnvalue_3))
  (bind _returnvalue_5 (CallFunction|LerpVector2D _viewportposition_3 _viewportposition _returnvalue_3))
  (bind _returnvalue_6 (CallFunction|LerpVector2D _returnvalue _returnvalue_2 Alpha))
  (bind (_x _y) (Math|Vector2D|BreakVector2D _returnvalue_6))
  (bind _returnvalue_7 (CallFunction|LerpVector2D _returnvalue_4 _returnvalue_5 _returnvalue_3))
  (return _returnvalue_6 (.yaw (Math|Rotator|FindLookatRotation (Math|Vector|MakeVector _x _y 0.0) (Math|Vector|MakeVector (.x _returnvalue_7) (.y _returnvalue_7) 0.0)))))

(fn GetWidgetTickSpacePosition
  (params (Widget :type Widget%20Object%20Reference))
  (return (.ViewportPosition (Class|SlateBlueprintLibrary|LocaltoViewport 0 (Class|Widget|GetTickSpaceGeometry Widget) (.translation (Variables|/Script/UMG.Widget|GetRenderTransform Widget))))))